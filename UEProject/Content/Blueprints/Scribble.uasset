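; Interactable scribble that is wiped away in four stages, one per interaction, and stays gone once its global flag is set in the game instance.
; Each interaction shows the next mesh layer and resumes a shared timeline that drives the Alpha parameter of four dynamic materials.
; A stage-end event stops the timeline, sets the next start time and advances the stage, saving the flag after the last.
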(event `self.ReceiveBeginPlay`
  (`parent.ReceiveBeginPlay`)
  (bind _asbp_game_instance (cast `/Game/Blueprints/Player/BP_GameInstance` (`GameplayStatics.GetGameInstance`)))
  (bind _output_get (set `self.GameInstanceRef` _asbp_game_instance))
  (if (`BlueprintSetLibrary.Set_Contains` (`/Game/Blueprints/Player/BP_GameInstance.GlobalFlags` _output_get) (`self.GlobalFlagName`))
    (`SceneComponent.SetVisibility` (`self.Scribble`) false true)
    (set `self.Enabled` false)
    (else
      (bind _returnvalue (`PrimitiveComponent.CreateDynamicMaterialInstance` (`self.ScribbleMesh1`) 0 "/Game/Assets/Materials/Level_1/ScribbleMaterial.ScribbleMaterial" "None"))
      (set `self.Material1` _returnvalue)
      (bind _returnvalue_2 (`PrimitiveComponent.CreateDynamicMaterialInstance` (`self.ScribbleMesh2`) 0 "/Game/Assets/Materials/Level_1/ScribbleMaterial.ScribbleMaterial" "None"))
      (set `self.Material2` _returnvalue_2)
      (bind _returnvalue_3 (`PrimitiveComponent.CreateDynamicMaterialInstance` (`self.ScribbleMesh3`) 0 "/Game/Assets/Materials/Level_1/ScribbleMaterial.ScribbleMaterial" "None"))
      (set `self.Material3` _returnvalue_3)
      (bind _returnvalue_4 (`PrimitiveComponent.CreateDynamicMaterialInstance` (`self.ScribbleMesh4`) 0 "/Game/Assets/Materials/Level_1/ScribbleMaterial.ScribbleMaterial" "None"))
      (set `self.Material4` _returnvalue_4)
      (`TimelineComponent.SetPlayRate` (`self.WipeTimeline`) (`self.WipeSpeed`)))))

(event `self.ReceiveTick`
  (params (DeltaSeconds :type "Float (single-precision)"))
  (`parent.ReceiveTick` DeltaSeconds)
  (if (`self.Animating`)
    (set `self.Animating` false)
    (bind (_direction _alpha1 _alpha2 _alpha3 _alpha4) (`Timeline|WipeTimeline` :`NewTime` (`self.Time`) :!label _label)
      (:`Update`
        (`MaterialInstanceDynamic.SetScalarParameterValue` (`self.Material1`) "Alpha" _alpha1)
        (`MaterialInstanceDynamic.SetScalarParameterValue` (`self.Material2`) "Alpha" _alpha2)
        (`MaterialInstanceDynamic.SetScalarParameterValue` (`self.Material3`) "Alpha" _alpha3)
        (`MaterialInstanceDynamic.SetScalarParameterValue` (`self.Material4`) "Alpha" _alpha4))
      (:`StageEnd`
        (`|ExecutionSequence`
          (:`then_0`
            (goto _label :!via `Stop`))
          (:`then_1`
            (switch `int` (`self.WipeStage`)
              (:`0`
                (set `self.Time` 1.001)
                (`SceneComponent.SetVisibility` (`self.ScribbleMesh1`) false false))
              (:`1`
                (set `self.Time` 2.001)
                (`SceneComponent.SetVisibility` (`self.ScribbleMesh2`) false false))
              (:`2`
                (set `self.Time` 3.001)
                (`SceneComponent.SetVisibility` (`self.ScribbleMesh3`) false false))
              (:`3`
                (set `self.Time` 4.001)))
            (bind _result (`/Engine/EditorBlueprintResources/StandardMacros.IncrementInt` (`self.WipeStage`))
              (:`  `
                (if (== _result 4)
                  (`BlueprintSetLibrary.Set_Add` (`/Game/Blueprints/Player/BP_GameInstance.GlobalFlags` (`self.GameInstanceRef`)) (`self.GlobalFlagName`))))))
          (:`then_2`
            (goto _label :!via `SetNewTime`)))))))

(event `self.OnInteract`
  (bind _wipestage (`self.WipeStage`))
  (if (< _wipestage 4)
    (set `self.Animating` true)
    (switch `int` _wipestage
      (:`0`
        (`SceneComponent.SetVisibility` (`self.ScribbleMesh2`) true false))
      (:`1`
        (`SceneComponent.SetVisibility` (`self.ScribbleMesh3`) true false))
      (:`2`
        (`SceneComponent.SetVisibility` (`self.ScribbleMesh4`) true false))
      (:`3`
        (set `self.UsableOnce` true)
        (set `self.Enabled` false)))))

(event `self.ReceiveActorBeginOverlap`
  (params (OtherActor :type "Actor Object Reference"))
  (`parent.ReceiveActorBeginOverlap` OtherActor))

(event `self.ReceiveActorEndOverlap`
  (params (OtherActor :type "Actor Object Reference"))
  (`parent.ReceiveActorEndOverlap` OtherActor))

(fn `UserConstructionScript`)