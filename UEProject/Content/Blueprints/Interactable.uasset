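; Base interactable actor that shows an icon widget and calls an empty OnInteract hook when the player presses Interact in range.
; Overlap events track range, while Tick turns the visible icon toward the player camera and rechecks eligibility.
; Optional facing check compares the actor's forward vector with the direction to the player using a dot product.
; Each use disables it, permanently if single-use, otherwise until a reuse delay ends and range is rechecked.
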(event `self.ReceiveBeginPlay`
  (`|ExecutionSequence`
    (:`then_0`
      (`self.EnableInput` (`GameplayStatics.GetPlayerController` 0))
      (bind _asbp_player_character (cast `/Game/Blueprints/Player/BP_PlayerCharacter` (`GameplayStatics.GetPlayerCharacter` 0)))
      (bind _output_get (set `self.PlayerRef` _asbp_player_character))
      (set `self.PlayerCameraRef` (`/Game/Blueprints/Player/BP_PlayerCharacter.PlayerCamera` _output_get)))
    (:`then_1`
      (bind _asicon_widget (cast `/Game/Blueprints/Widgets/IconWidget` (`WidgetComponent.GetUserWidgetObject` (`self.Widget`))))
      (`/Game/Blueprints/Widgets/IconWidget.SetImage` _asicon_widget (`self.IconImagePC`))
      (set `self.IconWidgetInstance` _asicon_widget))))

(event `self.ReceiveActorBeginOverlap`
  (params (OtherActor :type "Actor Object Reference"))
  (bind _asbp_player_character (cast `/Game/Blueprints/Player/BP_PlayerCharacter` OtherActor))
  (bind _return (`self.CompareFacing` _asbp_player_character))
  (if _return
    (`self.SetIconVisibility` true)
    (set `self.CanInteract` true))
  (set `self.InRange` true))

(event `self.ReceiveTick`
  (params (DeltaSeconds :type "Float (single-precision)"))
  (bind _widget (`self.Widget`))
  (`|ExecutionSequence`
    (:`then_0`
      (if (`self.Visible`)
        (`SceneComponent.K2_SetWorldRotation` _widget (`KismetMathLibrary.FindLookAtRotation` (`SceneComponent.K2_GetComponentLocation` _widget) (`SceneComponent.K2_GetComponentLocation` (`self.PlayerCameraRef`))) false false)))
    (:`then_1`
      (if (and (`self.InRange`) (`self.RequireFacing`) (`self.Enabled`))
        (bind _return (`self.CompareFacing` (`self.PlayerRef`)))
        (`self.SetIconVisibility` _return)
        (set `self.CanInteract` _return)))))

(event `self.ReceiveActorEndOverlap`
  (params (OtherActor :type "Actor Object Reference"))
  (cast `/Game/Blueprints/Player/BP_PlayerCharacter` OtherActor)
  (`self.SetIconVisibility` false)
  (set `self.CanInteract` false)
  (set `self.InRange` false))

(event `InputAction|Interact` :consume false
  (params (Key :type "Key Structure"))
  (bind _playerref (`self.PlayerRef`))
  (:`Pressed`
    (if (and (`self.CanInteract`) (`self.Enabled`))
      (set `self.Enabled` false)
      (`self.SetIconVisibility` false)
      (`self.OnInteract`)
      (if (not (`self.UsableOnce`))
        (`KismetSystemLibrary.Delay` (`self.ReuseTimer`))
        (set `self.Enabled` true)
        (bind _output_get (set `self.InRange` (`PrimitiveComponent.IsOverlappingActor` (`self.SphereTrigger`) _playerref)))
        (if _output_get
          (if (`self.RequireFacing`)
            (bind _return (`self.CompareFacing` _playerref))
            (bind _output_get_2 (set `self.CanInteract` _return))
            (`self.SetIconVisibility` _output_get_2)
            (else
              (set `self.CanInteract` true)
              (`self.SetIconVisibility` true))))))))

(fn `CompareFacing`
  (params (`Other Actor` :type "Actor Object Reference"))
  (returns (Return :type Boolean))
  (if (`self.RequireFacing`)
    (return (> (`KismetMathLibrary.Dot_VectorVector` (`KismetMathLibrary.Normal` (- (`self.K2_GetActorLocation` `Other Actor`) (`self.K2_GetActorLocation` self))) (`KismetMathLibrary.GetForwardVector` (`self.K2_GetActorRotation` self))) (- 1.0 (/ (`self.MaximumFacingAngle`) 360.0))))
    (else
      (return true))))

(fn `OnInteract`
  (return))

(fn `SetIconVisibility`
  (params (NewVisibility :type Boolean))
  (bind _visible (`self.Visible`))
  (bind _iconwidgetinstance (`self.IconWidgetInstance`))
  (if (!= NewVisibility _visible)
    (if _visible
      (bind _output_get (set `self.Visible` false))
      (`/Game/Blueprints/Widgets/IconWidget.SetEnabled` _iconwidgetinstance _output_get)
      (return)
      (else
        (bind _output_get_2 (set `self.Visible` true))
        (`/Game/Blueprints/Widgets/IconWidget.SetEnabled` _iconwidgetinstance _output_get_2)
        (return)))))

(fn `UserConstructionScript`)