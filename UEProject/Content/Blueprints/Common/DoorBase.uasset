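; Base door Blueprint that toggles open and closed on interact or trigger, playing sounds through the game instance.
; Timelines rotate the door mesh with an exponent-shaped lerp and optionally turn the handle on opening; collision can be disabled during motion.
; Swinging doors choose their direction from the dot product of player and arrow forward vectors.
; With auto-close enabled, Tick closes the door once the player moves beyond a 2D distance.
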(event `self.ReceiveBeginPlay`
  (bind _openspeed (`self.OpenSpeed`))
  (`parent.ReceiveBeginPlay`)
  (`TimelineComponent.SetPlayRate` (`self.DoorOpenClose`) _openspeed)
  (`TimelineComponent.SetPlayRate` (`self.HandleTurn`) _openspeed)
  (bind _bp_game_instance (`/Game/Blueprints/Common/MacroLibrary.MGetGameInstance`))
  (set `self.GameInstanceRef` _bp_game_instance)
  (bind _output_get (set `self.InitialRotation` (`SceneComponent.K2_GetComponentRotation` (`self.StaticMesh`))))
  (set `self.EndRotation` (`KismetMathLibrary.ComposeRotators` _output_get (`self.OpenRotation`)))
  (bind _output_get_2 (set `self.HandleInitialRotation` (`SceneComponent.RelativeRotation` (`self.HandleMesh`))))
  (set `self.HandleEndRotation` (`KismetMathLibrary.ComposeRotators` _output_get_2 (`self.HandleTurnRotation`)))
  (if (`self.AutoClose`)
    (set `self.DoorCenter` (`KismetSystemLibrary.GetComponentBounds` (`self.StaticMesh`)))))

(event `self.OnInteract`
  (bind _gameinstanceref (`self.GameInstanceRef`))
  (bind _staticmesh (`self.StaticMesh`))
  (bind _returnvalue (`self.K2_GetActorLocation` self))
  (if (`self.NoCollisionDuringMotion`)
    (`PrimitiveComponent.SetCollisionEnabled` _staticmesh "NoCollision"))
  (if (`self.IsOpen`)
    (`/Game/Blueprints/Player/BP_GameInstance.PlayLocalizedSound` _gameinstanceref _returnvalue (`self.CloseDoorSound`) 0.6 "NewEnumerator8" :!label _label)
    (set `self.IsOpen` false)
    (bind (_direction _float) (`Timeline|DoorOpenClose` :!via `Reverse` :!label _label_2)
      (:`Update`
        (`SceneComponent.K2_SetWorldRotation` (`self.StaticMesh`) (`KismetMathLibrary.RLerp` (`self.InitialRotation`) (`self.EndRotation`) (`KismetMathLibrary.MultiplyMultiply_FloatFloat` _float (`self.AnimationExponent`)) true) false false))
      (:`Finished`
        (`PrimitiveComponent.SetCollisionEnabled` _staticmesh "QueryAndPhysics")))
    (else
      (`self.SwingingDoorDirection`)
      (`/Game/Blueprints/Player/BP_GameInstance.PlayLocalizedSound` _gameinstanceref _returnvalue (`self.OpenDoorSound`) 0.6 "NewEnumerator8")
      (set `self.IsOpen` true)
      (`|ExecutionSequence`
        (:`then_0`
          (if (`self.HasHandle`)
            (bind (_direction_2 _float_2) (`Timeline|HandleTurn` :!via `PlayFromStart`)
              (:`Update`
                (`SceneComponent.K2_SetRelativeRotation` (`self.HandleMesh`) (`KismetMathLibrary.RLerp` (`self.HandleInitialRotation`) (`self.HandleEndRotation`) _float_2 true) false false)))))
        (:`then_1`
          (goto _label_2))))))

(event `/Game/Blueprints/Common/Interfaces/ITriggerable.TriggerEvent`
  (params (TriggerObject :type "/Game/Blueprints/Common/EventTrigger Object Reference"))
  (`self.OnInteract`))

(event `self.ReceiveTick`
  (params (DeltaSeconds :type "Float (single-precision)"))
  (if (and (`self.AutoClose`) (`self.IsOpen`))
    (if (> (`KismetMathLibrary.Vector_Distance2D` (`self.K2_GetActorLocation` (`/Game/Blueprints/Player/BP_GameInstance.PlayerCharacterRef` (`self.GameInstanceRef`))) (`self.DoorCenter`)) (`self.AutoCloseDistance`))
      (`|ExecutionSequence`
        (:`then_0`
          (goto _label))
        (:`then_1`
          _))))
  (`parent.ReceiveTick` DeltaSeconds))

(fn `SwingingDoorDirection`
  (bind _openrotation (`self.OpenRotation`))
  (bind _initialrotation (`self.InitialRotation`))
  (if (`self.SwingingDoor`)
    (bind _bp_player_character (`/Game/Blueprints/Common/MacroLibrary.MGetPlayerCharacter`))
    (if (< (`KismetMathLibrary.Dot_VectorVector` (`self.GetActorForwardVector` _bp_player_character) (`SceneComponent.GetForwardVector` (`self.Arrow`))) 0.0)
      (set `self.EndRotation` (`KismetMathLibrary.ComposeRotators` _initialrotation (* _openrotation -1.0)))
      (else
        (set `self.EndRotation` (`KismetMathLibrary.ComposeRotators` _initialrotation _openrotation))))))

(fn `UserConstructionScript`
  (`parent.UserConstructionScript`))