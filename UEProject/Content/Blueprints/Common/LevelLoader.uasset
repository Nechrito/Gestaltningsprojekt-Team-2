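; Level streaming manager that registers itself with BP_GameInstance and creates the main menu widget when one is set.
; Queued load and unload requests run through a recursive pass that tracks loaded levels in a set.
; An optional Loading_Screen sublevel covers the transition, with a timer for minimum display time.
; Removing that screen enables the player character, or gives UI focus to the menu when one is set.
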(event `self.ReceiveBeginPlay`
  (bind _mainmenuwidget (`self.MainMenuWidget`))
  (bind _asbp_game_instance (cast `/Game/Blueprints/Player/BP_GameInstance` (`GameplayStatics.GetGameInstance`)))
  (set `/Game/Blueprints/Player/BP_GameInstance.LevelLoaderInstance` self _asbp_game_instance)
  (if (`KismetSystemLibrary.IsValidClass` _mainmenuwidget)
    (bind _returnvalue (`|CreateWidget` _mainmenuwidget (`GameplayStatics.GetPlayerControllerFromID` 0)))
    (`UserWidget.AddToViewport` _returnvalue 0)
    (set `self.MainMenuRef` _returnvalue)))

(event `LoadLevel`
  (params (LevelName :type Name))
  ;[1 1 1] Load / Unload Level
)

(event `UnloadLevel`
  (params (LevelName :type Name))
  (bind _loadedlevels (`self.LoadedLevels`))
  ;[1 1 1] Load / Unload Level
  (if (`BlueprintSetLibrary.Set_Contains` _loadedlevels LevelName)
    (`GameplayStatics.UnloadStreamLevel` LevelName)
    (`BlueprintSetLibrary.Set_Remove` _loadedlevels LevelName)))

(event `LoadEvent`
  ;[1 1 1] Begin Loading Queued Levels
  (if (`self.LoadTimer`)
    (set `self.LoadTimer` false))
  (`self.RemoveLoadingScreen`))

(event `BeginLoad`
  (params (ShowLoadingScreen :type Boolean))
  ;[1 1 1] Begin Loading Queued Levels
  (if (`self.LoadingScreenEnabled`)
    (set `self.LoadTimer` true :!label _label)
    (`KismetSystemLibrary.K2_SetTimerDelegate` (delegate `LoadEvent`) (`self.LoadScreenMinDuration`))
    (else
      (bind _output_get (set `self.LoadingScreenEnabled` ShowLoadingScreen))
      (if _output_get
        (`GameplayStatics.LoadStreamLevel` "Loading_Screen" true true)
        (goto _label)
        (else
          _))))
  (set `self.Index` 0)
  (`self.LoadRecursive`))

(event `LoadRecursive`
  (bind _loadedlevels (`self.LoadedLevels`))
  (bind _index (`self.Index`))
  (bind _loadqueue (`self.LoadQueue`))
  (bind (_levelname _action) (break `/Game/Blueprints/Common/Structs/LevelStreamData` (`|GetArrayItem` _loadqueue _index)))
  (bind _returnvalue (`BlueprintSetLibrary.Set_Contains` _loadedlevels _levelname))
  ;[1 1 1] Comment
  (if (< _index (`KismetArrayLibrary.Array_Length` _loadqueue))
    (switch `/Game/Blueprints/Common/Enum/LevelStreamAction` _action
      (:`NewEnumerator0`
        (if (not _returnvalue)
          (`GameplayStatics.LoadStreamLevel` _levelname true)
          (`BlueprintSetLibrary.Set_Add` _loadedlevels _levelname)))
      (:`NewEnumerator1`
        (if _returnvalue
          (`GameplayStatics.UnloadStreamLevel` _levelname)
          (`BlueprintSetLibrary.Set_Remove` _loadedlevels _levelname))))
    (`/Engine/EditorBlueprintResources/StandardMacros.IncrementInt` _index
      (:`  `
        (`self.LoadRecursive`)))
    (else
      (`KismetArrayLibrary.Array_Clear` _loadqueue)
      (if (`self.LoadTimer`)
        (set `self.LoadTimer` false)
        (else
          (`self.RemoveLoadingScreen`))))))

(event `UnhideLevel`
  (params (LevelName :type Name))
  (set `LevelStreaming.bShouldBeVisible` true (`GameplayStatics.GetStreamingLevel` LevelName)))

(event `UnhideLoadedLevels`
  (bind _result (`BlueprintSetLibrary.Set_ToArray` (`self.LoadedLevels`)))
  (for _array_element _result
    (bind _returnvalue (`GameplayStatics.GetStreamingLevel` _array_element))
    (if (`KismetSystemLibrary.IsValid` _returnvalue)
      (set `LevelStreaming.bShouldBeVisible` true _returnvalue))))

(event `RemoveLoadingScreen`
  (bind _returnvalue (`GameplayStatics.GetPlayerController` 0))
  (if (`self.LoadingScreenEnabled`)
    (`Widget.RemoveFromParent` (`self.LoadScreenWidget`))
    (`GameplayStatics.UnloadStreamLevel` "Loading_Screen")
    (set `self.LoadingScreenEnabled` false)
    (if (not (`KismetSystemLibrary.IsValidClass` (`self.MainMenuWidget`)))
      (bind _asbp_player_character (cast `/Game/Blueprints/Player/BP_PlayerCharacter` (`GameplayStatics.GetPlayerCharacter` 0)))
      (`/Game/Blueprints/Player/BP_PlayerCharacter.SetPlayerEnabled` _asbp_player_character true)
      (else
        (bind _asifocusable (cast `/Game/Blueprints/Common/Interfaces/IFocusable` (`self.MainMenuRef`)))
        (bind _widget (`/Game/Blueprints/Widgets/Main_Menu.GetPreferredFocus` _asifocusable))
        (`WidgetBlueprintLibrary.SetInputMode_UIOnlyEx` _returnvalue _widget)
        (set `PlayerController.bShowMouseCursor` true _returnvalue)))))

(event `ShowLoadingScreen`
  (set `self.LoadingScreenEnabled` true)
  (`GameplayStatics.LoadStreamLevel` "Loading_Screen" true))

(event `BeginUnloadAll`
  (bind _loadedlevels (`self.LoadedLevels`))
  (bind _output_get (set `self.Index` 0))
  (bind _result (`BlueprintSetLibrary.Set_ToArray` _loadedlevels))
  (`GameplayStatics.UnloadStreamLevel` (`|GetArrayItem` _result) true :!label _label_2)
  (bind _result_2 (`/Engine/EditorBlueprintResources/StandardMacros.IncrementInt` _output_get)
    (:`  `
      (if (< _result_2 (`KismetArrayLibrary.Array_Length` _result))
        (goto _label_2)
        (else
          (`BlueprintSetLibrary.Set_Clear` _loadedlevels))))))

(fn `EnqueueLevel`
  (params (LevelData :type "/Game/Blueprints/Common/Structs/LevelStreamData Structure"))
  (`KismetArrayLibrary.Array_Add` (`self.LoadQueue`) LevelData)
  (return))

(fn `IsLevelLoaded`
  (params (LevelName :type Name))
  (returns (Return :type Boolean))
  (return (`BlueprintSetLibrary.Set_Contains` (`self.LoadedLevels`) LevelName)))

(fn `UserConstructionScript`)