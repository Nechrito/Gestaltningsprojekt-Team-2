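; Saveable actor that swaps static mesh objects in the level while the player looks away from it.
; Hides Objects on BeginPlay and arms itself after a delay or through TriggerEvent.
; Tick uses a 2D camera dot product and minimum distance check to show Objects, hide HideObjects and disarm.
; Loading replays the swap if HasTriggered is saved true, though the Tick trigger sets that flag false.
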(event `self.ReceiveBeginPlay`
  (bind _bp_game_instance (`/Game/Blueprints/Common/MacroLibrary.MGetGameInstance`))
  (set `self.GameInstanceRef` _bp_game_instance)
  (`/Game/Blueprints/Common/MacroLibrary.MRegisterSaveable`)
  (for _array_element (`self.Objects`)
    (bind _staticmeshcomponent (`StaticMeshActor.StaticMeshComponent` _array_element))
    (`SceneComponent.SetVisibility` _staticmeshcomponent false true)
    (`PrimitiveComponent.SetCollisionEnabled` _staticmeshcomponent "NoCollision"))
  (`KismetSystemLibrary.Delay` 2.0)
  (set `self.IsEnabled` true))

(event `self.ReceiveTick`
  (params (DeltaSeconds :type "Float (single-precision)"))
  (bind _returnvalue (`self.K2_GetActorLocation`))
  (bind _playercharacterref (`/Game/Blueprints/Player/BP_GameInstance.PlayerCharacterRef` (`self.GameInstanceRef`)))
  (bind _returnvalue_2 (`self.K2_GetActorLocation` _playercharacterref))
  (if (`self.IsEnabled`)
    (if (and (> (`KismetMathLibrary.DotProduct2D` (`KismetMathLibrary.Normal2D` (`KismetMathLibrary.Conv_VectorToVector2D` (- _returnvalue_2 _returnvalue))) (`KismetMathLibrary.Conv_VectorToVector2D` (`SceneComponent.GetForwardVector` (`/Game/Blueprints/Player/BP_PlayerCharacter.PlayerCamera` _playercharacterref)))) 0.75) (> (`KismetMathLibrary.Vector_Distance2D` _returnvalue _returnvalue_2) (`self.MinimumDistance`)))
      (set `self.IsEnabled` false)
      (set `self.HasTriggered` false)
      (for _array_element (`self.Objects`) :!label _label
        (bind _staticmeshcomponent (`StaticMeshActor.StaticMeshComponent` _array_element))
        (`SceneComponent.SetVisibility` _staticmeshcomponent true true)
        (`PrimitiveComponent.SetCollisionEnabled` _staticmeshcomponent "QueryAndPhysics"))
      (for _array_element_2 (`self.HideObjects`)
        (bind _staticmeshcomponent_2 (`StaticMeshActor.StaticMeshComponent` _array_element_2))
        (`SceneComponent.SetVisibility` _staticmeshcomponent_2 false false)
        (`PrimitiveComponent.SetCollisionEnabled` _staticmeshcomponent_2 "NoCollision")))))

(event `/Game/Blueprints/Common/Interfaces/ISaveable.LoadState`
  (params (Data :type "/Game/Blueprints/Common/Structs/SaveableData Structure"))
  (bind (_name _transform _isactivated _isdestroyed) (break `/Game/Blueprints/Common/Structs/SaveableData` Data))
  (set `self.IsEnabled` _isactivated)
  (bind _output_get (set `self.HasTriggered` _isdestroyed))
  (if _output_get
    (goto _label)))

(event `/Game/Blueprints/Common/Interfaces/ITriggerable.TriggerEvent`
  (params (TriggerObject :type "/Game/Blueprints/Common/EventTrigger Object Reference"))
  (set `self.IsEnabled` true))

(fn `SaveState`
  (returns (Data :type "/Game/Blueprints/Common/Structs/SaveableData Structure"))
  (return (make `/Game/Blueprints/Common/Structs/SaveableData` (`KismetStringLibrary.Conv_StringToName` (`KismetSystemLibrary.GetObjectName` self)) "0.000000,0.000000,0.000000|0.000000,0.000000,0.000000|1.000000,1.000000,1.000000" (`self.IsEnabled`) (`self.HasTriggered`))))

(fn `UserConstructionScript`)