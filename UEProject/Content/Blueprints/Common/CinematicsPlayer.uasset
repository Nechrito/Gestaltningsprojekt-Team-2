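; CinematicsPlayer is an actor that plays an intro or ending level sequence, then starts or ends the game through the game instance.
; On BeginPlay it enables input, plays the sequence after a configurable delay, and toggles a post-process Multiply parameter from zero to one around it.
; Pressing Pause skips the cinematic, triggering the same transition immediately and stopping the sequence a second later, with a Skip flag preventing a double call.
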(event `self.ReceiveBeginPlay`
  (bind _sequenceplayer (`LevelSequenceActor.SequencePlayer` (`self.CinematicSequence`)))
  (`KismetMaterialLibrary.SetScalarParameterValue` "/Game/Assets/Materials/PostProcessMaterialParameters.PostProcessMaterialParameters" "Multiply")
  (bind _bp_game_instance (`/Game/Blueprints/Common/MacroLibrary.MGetGameInstance`))
  (bind _output_get (set `self.GameInstanceRef` _bp_game_instance))
  (`self.EnableInput` (`/Game/Blueprints/Player/BP_PlayerCharacter.PlayerControllerRef` (`/Game/Blueprints/Player/BP_GameInstance.PlayerCharacterRef` _output_get)))
  (add `MovieSceneSequencePlayer.OnFinished` _sequenceplayer (delegate `OnCinematicFinished`))
  (`KismetSystemLibrary.Delay` (`self.Delay`))
  (`MovieSceneSequencePlayer.Play` _sequenceplayer)
  (`KismetMaterialLibrary.SetScalarParameterValue` "/Game/Assets/Materials/PostProcessMaterialParameters.PostProcessMaterialParameters" "Multiply" 1.0))

(event `OnCinematicFinished`
  (bind _gameinstanceref (`self.GameInstanceRef`))
  (if (`self.Skip`)
    _
    (elif (`self.Ending`)
      (`/Game/Blueprints/Player/BP_GameInstance.EndGame` _gameinstanceref)
      (else
        (`/Game/Blueprints/Player/BP_GameInstance.StartGame` _gameinstanceref)))))

(event `InputAction|Pause`
  (params (Key :type "Key Structure"))
  (bind _gameinstanceref (`self.GameInstanceRef`))
  (:`Pressed`
    (if (not (`self.Skip`))
      (set `self.Skip` true)
      (if (`self.Ending`)
        (`/Game/Blueprints/Player/BP_GameInstance.EndGame` _gameinstanceref)
        (else
          (`/Game/Blueprints/Player/BP_GameInstance.StartGame` _gameinstanceref)))
      (`KismetSystemLibrary.Delay` 1.0)
      (`MovieSceneSequencePlayer.Stop` (`LevelSequenceActor.SequencePlayer` (`self.CinematicSequence`))))))

(fn `UserConstructionScript`)