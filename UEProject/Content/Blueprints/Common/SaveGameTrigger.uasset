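; One-shot save trigger actor that saves the game through BP_GameInstance when BP_PlayerCharacter first overlaps it.
; The overlap sets a Triggered flag and calls Disable on every chained trigger before saving.
; SaveState records that flag under the actor's object name.
; LoadState has an empty body, while Disable assigns Triggered from the LoadState Data's IsActivated value.
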(event `self.ReceiveBeginPlay`)

(event `self.ReceiveActorBeginOverlap`
  (params (OtherActor :type "Actor Object Reference"))
  (if (not (`self.Triggered`))
    (cast `/Game/Blueprints/Player/BP_PlayerCharacter` OtherActor)
    (set `self.Triggered` true)
    (for _array_element (`self.ChainedTriggers`)
      (`self.Disable` _array_element))
    (bind _asbp_game_instance (cast `/Game/Blueprints/Player/BP_GameInstance` (`GameplayStatics.GetGameInstance`)))
    (`/Game/Blueprints/Player/BP_GameInstance.SaveGame` _asbp_game_instance)))

(event `Disable`
  (set `self.Triggered` (`.IsActivated_8_92C3EF144F16EB23865748A86EEA5CCD` (break `/Game/Blueprints/Common/Structs/SaveableData` (stale `/Game/Blueprints/Common/Interfaces/ISaveable.LoadState` Data)))))

(event `/Game/Blueprints/Common/Interfaces/ISaveable.LoadState`
  (params (Data :type "/Game/Blueprints/Common/Structs/SaveableData Structure")))

(fn `SaveState`
  (returns (Data :type "/Game/Blueprints/Common/Structs/SaveableData Structure"))
  (return (make `/Game/Blueprints/Common/Structs/SaveableData` (`KismetStringLibrary.Conv_StringToName` (`KismetSystemLibrary.GetObjectName` self)) "0.000000,0.000000,0.000000|0.000000,0.000000,0.000000|1.000000,1.000000,1.000000" (`self.Triggered`))))

(fn `UserConstructionScript`)