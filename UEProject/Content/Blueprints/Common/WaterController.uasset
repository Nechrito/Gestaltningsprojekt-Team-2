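; Water volume controller that drives the player's underwater post-processing and the splash feedback when entering or leaving water.
; At BeginPlay it fits surface and post-process boxes to a physics volume and records the surface height.
; Surface overlaps use vertical velocity to toggle submersion, notify the game instance and trigger impact-scaled particles with sound.
; While overlapping, Tick sets material-collection submersion and blur from camera depth, reduced near the surface when looking up.
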(event `self.ReceiveBeginPlay`
  (bind _surfacecollision (`self.SurfaceCollision`))
  (bind _postprocess (`self.PostProcess`))
  (bind _returnvalue (* (`self.SurfaceThickness`) 0.5))
  (bind _returnvalue_2 (* (`self.PostProcessDepth`) 0.5))
  (bind (_origin _boxextent) (`KismetSystemLibrary.GetComponentBounds` (`Brush.BrushComponent` (`self.PhysicsVolume`))))
  (bind _x (.x _boxextent))
  (bind _y (.y _boxextent))
  (bind _z (.z _boxextent))
  (bind _bp_game_instance (`/Game/Blueprints/Common/MacroLibrary.MGetGameInstance`))
  (bind _output_get (set `self.GameInstanceRef` _bp_game_instance))
  (`self.EnableInput` (`/Game/Blueprints/Player/BP_PlayerCharacter.PlayerControllerRef` (`/Game/Blueprints/Player/BP_GameInstance.PlayerCharacterRef` _output_get)))
  (`SceneComponent.K2_SetWorldLocation` (`self.PostProcessBounds`) (+ _origin (`KismetMathLibrary.MakeVector` 0.0 0.0 (* _returnvalue_2 -1.0))) false true)
  (`BoxComponent.SetBoxExtent` _surfacecollision (`KismetMathLibrary.MakeVector` _x _y _returnvalue) true)
  (`SceneComponent.K2_SetRelativeLocation` _surfacecollision (`KismetMathLibrary.MakeVector` 0.0 0.0 (+ (- (+ _z _returnvalue_2) _returnvalue) (`self.SurfaceOffset`))) false true)
  (`BoxComponent.SetBoxExtent` (`self.PostProcessBounds`) (`KismetMathLibrary.MakeVector` _x _y (- _z _returnvalue_2)) true)
  (set `PostProcessComponent.bUnbound` false _postprocess)
  (set `PostProcessComponent.Settings` (`self.UnderwaterPostProcessing`) _postprocess)
  (`self.UpdateSurface`))

(event `self.ReceiveTick`
  (params (DeltaSeconds :type "Float (single-precision)"))
  (bind _postprocesssurfacethickness (`self.PostProcessSurfaceThickness`))
  (bind _playercharacterref (`/Game/Blueprints/Player/BP_GameInstance.PlayerCharacterRef` (`self.GameInstanceRef`)))
  (bind _returnvalue (- (+ (`self.SurfaceLevel`) (`self.PostProcessSurfaceOffset`)) (.z (`SceneComponent.K2_GetComponentLocation` (`/Game/Blueprints/Player/BP_PlayerCharacter.PlayerCamera` _playercharacterref)))))
  (bind _returnvalue_2 (/ (`KismetMathLibrary.FClamp` _returnvalue 0.0 _postprocesssurfacethickness) _postprocesssurfacethickness))
  (bind _returnvalue_3 (`KismetMathLibrary.FClamp` (- _returnvalue_2 (`KismetMathLibrary.FClamp` (.z (`SceneComponent.GetForwardVector` (`/Game/Blueprints/Player/BP_PlayerCharacter.PlayerCamera` _playercharacterref)))))))
  (if (`self.Colliding`)
    (if (> _returnvalue 5.0)
      (`KismetMaterialLibrary.SetScalarParameterValue` "/Game/Assets/Materials/PostProcessMaterialParameters.PostProcessMaterialParameters" "UnderwaterSubmersion" _returnvalue_2)
      (`KismetMaterialLibrary.SetScalarParameterValue` "/Game/Assets/Materials/PostProcessMaterialParameters.PostProcessMaterialParameters" "BlurRadius" (* _returnvalue_2 1.5))
      (else
        (`KismetMaterialLibrary.SetScalarParameterValue` "/Game/Assets/Materials/PostProcessMaterialParameters.PostProcessMaterialParameters" "UnderwaterSubmersion" _returnvalue_3)
        (`KismetMaterialLibrary.SetScalarParameterValue` "/Game/Assets/Materials/PostProcessMaterialParameters.PostProcessMaterialParameters" "BlurRadius" (* 1.5 _returnvalue_3))))))

(event `self.SurfaceCollision.OnComponentBeginOverlap`
  (params (OverlappedComponent :type "PrimitiveComponent Object Reference") (OtherActor :type "Actor Object Reference") (OtherComp :type "PrimitiveComponent Object Reference") (OtherBodyIndex :type Integer) (bFromSweep :type Boolean) (SweepResult :type "HitResult Structure (by ref)"))
  (bind _asbp_player_character (cast `/Game/Blueprints/Player/BP_PlayerCharacter` OtherActor))
  (`self.CheckSurface` _asbp_player_character))

(event `self.SurfaceCollision.OnComponentEndOverlap`
  (params (OverlappedComponent :type "PrimitiveComponent Object Reference") (OtherActor :type "Actor Object Reference") (OtherComp :type "PrimitiveComponent Object Reference") (OtherBodyIndex :type Integer))
  (bind _asbp_player_character (cast `/Game/Blueprints/Player/BP_PlayerCharacter` OtherActor))
  (`self.CheckSurface` _asbp_player_character))

(event `UpdateSurface`
  (bind _physicsvolume (`self.PhysicsVolume`))
  (bind _returnvalue (+ (.z (`self.K2_GetActorLocation` _physicsvolume)) (.z (`.BoxExtent` (`KismetSystemLibrary.GetComponentBounds` (`Brush.BrushComponent` _physicsvolume))))))
  (`KismetMaterialLibrary.SetScalarParameterValue` "/Game/Assets/Materials/PostProcessMaterialParameters.PostProcessMaterialParameters" "UnderwaterSurfaceLevel" _returnvalue)
  (set `self.SurfaceLevel` _returnvalue))

(event `CheckSurface`
  (params (PlayerCharacter :type "/Game/Blueprints/Player/BP_PlayerCharacter Object Reference"))
  (bind _gameinstanceref (`self.GameInstanceRef`))
  (bind _gameinstanceref_2 (`self.GameInstanceRef`))
  (bind _splashparticles (`self.SplashParticles`))
  (bind _z (.z (`CharacterMovementComponent.GetLastUpdateVelocity` (`Character.CharacterMovement` PlayerCharacter))))
  (bind _feet (`/Game/Blueprints/Player/BP_PlayerCharacter.Feet` (`/Game/Blueprints/Player/BP_GameInstance.PlayerCharacterRef` _gameinstanceref_2)))
  (bind _returnvalue (/ (`KismetMathLibrary.FClamp` _z 0.0 20.0) 20.0))
  (bind _returnvalue_2 (/ (`KismetMathLibrary.Abs` (`KismetMathLibrary.FClamp` _z 0.0 -20.0)) 20.0))
  (if (`self.Submerged`)
    (if (> _z 0.0)
      (set `self.Submerged` false)
      (set `/Game/Blueprints/Player/BP_PlayerCharacter.Submerged` false PlayerCharacter)
      (`/Game/Blueprints/Player/BP_GameInstance.LeaveWater` _gameinstanceref _returnvalue)
      (`SceneComponent.K2_SetWorldLocation` _splashparticles (`self.K2_GetActorLocation` PlayerCharacter) false true)
      (`FXSystemComponent.SetEmitterEnable` _splashparticles "None" true)
      (`FXSystemComponent.SetFloatParameter` _splashparticles "Impact" _returnvalue)
      (`/Game/Blueprints/Player/BP_GameInstance.PlayCharacterSound` _gameinstanceref_2 _feet "NewEnumerator23" 1.0 "NewEnumerator8"))
    (elif (< _z 0.0)
      (set `self.Submerged` true)
      (set `/Game/Blueprints/Player/BP_PlayerCharacter.Submerged` true PlayerCharacter)
      (`/Game/Blueprints/Player/BP_GameInstance.EnterWater` _gameinstanceref _returnvalue_2)
      (`SceneComponent.K2_SetWorldLocation` _splashparticles (`self.K2_GetActorLocation` PlayerCharacter) false true)
      (`FXSystemComponent.SetEmitterEnable` _splashparticles "None" true)
      (`FXSystemComponent.SetFloatParameter` _splashparticles "Impact" _returnvalue_2)
      (`/Game/Blueprints/Player/BP_GameInstance.PlayCharacterSound` _gameinstanceref_2 _feet "NewEnumerator23" 1.0 "NewEnumerator8"))))

(event `self.PostProcessBounds.OnComponentBeginOverlap`
  (params (OverlappedComponent :type "PrimitiveComponent Object Reference") (OtherActor :type "Actor Object Reference") (OtherComp :type "PrimitiveComponent Object Reference") (OtherBodyIndex :type Integer) (bFromSweep :type Boolean) (SweepResult :type "HitResult Structure (by ref)"))
  (cast `/Game/Blueprints/Player/BP_PlayerCharacter` OtherActor)
  (set `self.Colliding` true))

(event `self.PostProcessBounds.OnComponentEndOverlap`
  (params (OverlappedComponent :type "PrimitiveComponent Object Reference") (OtherActor :type "Actor Object Reference") (OtherComp :type "PrimitiveComponent Object Reference") (OtherBodyIndex :type Integer))
  (cast `/Game/Blueprints/Player/BP_PlayerCharacter` OtherActor)
  (set `self.Colliding` false))

(fn `NewFunction_0`)

(fn `SetSubmerged`
  (set `self.Colliding` true)
  (set `self.Submerged` true))

(fn `UserConstructionScript`)