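; Base actor for interactable objects that shows an icon when the player can use them and fires an empty OnInteract hook on the Interact input.
; A sphere trigger sets range, then dot-product tests check optional one- or two-sided facing and whether the icon lies within the camera's view.
; Tick updates visibility and turns the icon toward the camera.
; Use is delayed briefly, then either locks or re-arms after a reuse timer.
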(event `self.ReceiveBeginPlay`
  (`|ExecutionSequence`
    (:`then_0`
      (`self.EnableInput` (`GameplayStatics.GetPlayerController` 0))
      (bind _asbp_player_character (cast `/Game/Blueprints/Player/BP_PlayerCharacter` (`GameplayStatics.GetPlayerCharacter` 0)))
      (bind _output_get (set `self.PlayerRef` _asbp_player_character))
      (set `self.PlayerCameraRef` (`/Game/Blueprints/Player/BP_PlayerCharacter.PlayerCamera` _output_get)))
    (:`then_1`
      (bind _asicon_widget (cast `/Game/Blueprints/Widgets/IconWidget` (`WidgetComponent.GetUserWidgetObject` (`self.Widget`))))
      (`/Game/Blueprints/Widgets/IconWidget.SetImage` _asicon_widget (`self.InteractIcon`))
      (set `self.IconWidgetInstance` _asicon_widget))))

(event `CheckOverlap`
  (if (`PrimitiveComponent.IsOverlappingActor` (`self.SphereTrigger`) (`self.PlayerRef`))
    (if (and (not (`self.InMotion`)) (`self.CanUse`)) :!label _label
      (cast `/Game/Blueprints/Player/BP_PlayerCharacter` (stale `self.ReceiveActorBeginOverlap` OtherActor))
      (bind _return (`self.CompareFacing`))
      (if _return
        (bind _in_view (`self.CheckViewBoundaries`))
        (if _in_view
          (`self.SetIconVisibility` true)
          (set `self.InView` true)))
      (set `self.InRange` true)
      (`self.SetDisabledState`))))

(event `self.ReceiveActorBeginOverlap`
  (params (OtherActor :type "Actor Object Reference"))
  (goto _label))

(event `self.ReceiveTick`
  (params (DeltaSeconds :type "Float (single-precision)"))
  (bind _widgetnode (`self.WidgetNode`))
  (bind _returnvalue (not (`self.InMotion`)))
  (`|ExecutionSequence`
    (:`then_0`
      (if (and (`self.Visible`) _returnvalue)
        (`SceneComponent.K2_SetWorldRotation` _widgetnode (`KismetMathLibrary.MakeRotator` 0.0 (.pitch (`KismetMathLibrary.FindLookAtRotation` (`SceneComponent.K2_GetComponentLocation` _widgetnode) (`SceneComponent.K2_GetComponentLocation` (`self.PlayerCameraRef`)))) (.yaw (`KismetMathLibrary.FindLookAtRotation` (`SceneComponent.K2_GetComponentLocation` _widgetnode) (`SceneComponent.K2_GetComponentLocation` (`self.PlayerCameraRef`))))) false false)))
    (:`then_1`
      (if (and (`self.InRange`) (`self.CanUse`) _returnvalue)
        (if (`self.RequireFacing`)
          (bind _return (`self.CompareFacing`))
          (if _return
            (bind _in_view (`self.CheckViewBoundaries` :!label _label_2))
            (if _in_view
              (`self.SetIconVisibility` true)
              (set `self.InView` true)
              (else
                (`self.SetIconVisibility` false :!label _label_3)
                (set `self.InView` false)))
            (else
              (goto _label_3)))
          (else
            (goto _label_2)))))))

(event `self.ReceiveActorEndOverlap`
  (params (OtherActor :type "Actor Object Reference"))
  (cast `/Game/Blueprints/Player/BP_PlayerCharacter` OtherActor)
  (`self.SetIconVisibility` false)
  (set `self.InView` false)
  (set `self.InRange` false))

(event `InputAction|Interact` :consume false
  (params (Key :type "Key Structure"))
  (:`Pressed`
    (if (and (`self.InView`) (`self.CanUse`) (`self.InRange`) (not (`self.Disabled`)))
      (set `self.CanUse` false)
      (`self.SetIconVisibility` false)
      (`|ExecutionSequence`
        (:`then_0`
          (`KismetSystemLibrary.Delay` 0.32)
          (`self.OnInteract`))
        (:`then_1`
          (if (not (`self.UsableOnce`))
            (`KismetSystemLibrary.Delay` (`self.ReuseTimer`))
            (if (not (`self.UsableOnce`))
              (set `self.CanUse` true)
              (bind _output_get (set `self.InRange` (`PrimitiveComponent.IsOverlappingActor` (`self.SphereTrigger`) (`self.PlayerRef`))))
              (if _output_get
                (if (`self.RequireFacing`)
                  (bind _return (`self.CompareFacing`))
                  (bind _output_get_2 (set `self.InView` _return))
                  (`self.SetIconVisibility` _output_get_2)
                  (else
                    (set `self.InView` true)
                    (`self.SetIconVisibility` true)))))))))))

(event `OnInteract`)

(fn `CheckViewBoundaries`
  (returns (`In View` :type Boolean))
  (bind _playercamera (`/Game/Blueprints/Player/BP_PlayerCharacter.PlayerCamera` (`self.PlayerRef`)))
  (return (> (`KismetMathLibrary.Dot_VectorVector` (`KismetMathLibrary.Normal` (- (`SceneComponent.K2_GetComponentLocation` (`self.WidgetNode`)) (`SceneComponent.K2_GetComponentLocation` _playercamera))) (`SceneComponent.GetForwardVector` _playercamera)) (- 1.0 (/ (`self.ActiveFOV`) 360.0)))))

(fn `CompareFacing`
  (returns (Return :type Boolean))
  (bind _returnvalue (- 1.0 (/ (`self.MaximumFacingAngle`) 360.0)))
  (bind _returnvalue_2 (`KismetMathLibrary.Dot_VectorVector` (`KismetMathLibrary.Normal` (- (`SceneComponent.K2_GetComponentLocation` (`self.PlayerCameraRef`)) (`SceneComponent.K2_GetComponentLocation` (`self.Billboard`)))) (`SceneComponent.GetForwardVector` (`self.Arrow`))))
  (bind _returnvalue_3 (> _returnvalue_2 _returnvalue))
  (if (`self.RequireFacing`)
    (if (`self.TwoSided`)
      (return (or _returnvalue_3 (> (`KismetMathLibrary.Abs` _returnvalue_2) _returnvalue)))
      (else
        (return _returnvalue_3)))
    (else
      (return true))))

(fn `SetDisabledState`
  (bind _iconwidgetinstance (`self.IconWidgetInstance`))
  (if (`self.ShowDisabledIcon`)
    (if (`self.Disabled`)
      (`/Game/Blueprints/Widgets/IconWidget.SetImage` _iconwidgetinstance (`self.DisabledIcon`))
      (else
        (`/Game/Blueprints/Widgets/IconWidget.SetImage` _iconwidgetinstance (`self.InteractIcon`))))
    (return)))

(fn `SetIconVisibility`
  (params (NewVisibility :type Boolean))
  (bind _visible (`self.Visible`))
  (bind _iconwidgetinstance (`self.IconWidgetInstance`))
  (if (!= NewVisibility _visible)
    (if _visible
      (bind _output_get (set `self.Visible` false))
      (`/Game/Blueprints/Widgets/IconWidget.SetEnabled` _iconwidgetinstance _output_get)
      (return)
      (else
        (bind _output_get_2 (set `self.Visible` true))
        (`/Game/Blueprints/Widgets/IconWidget.SetEnabled` _iconwidgetinstance _output_get_2)
        (return)))))

(fn `UserConstructionScript`)