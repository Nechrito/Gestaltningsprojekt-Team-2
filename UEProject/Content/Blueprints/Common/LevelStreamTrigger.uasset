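; Level streaming trigger actor that loads a list of levels through the LevelLoader found in the world.
; It either loads on BeginPlay, disabling its overlap events, or when BP_PlayerCharacter overlaps it, optionally only once.
; An optional direction limit compares the arrow and player forward vectors by dot product.
; Each load enqueues every level, then begins loading with an optional loading screen.
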(event `self.ReceiveBeginPlay`
  (bind _levelloaderinstance (`self.LevelLoaderInstance`))
  (bind _returnvalue (`GameplayStatics.GetActorOfClass` "/Game/Blueprints/Common/LevelLoader.LevelLoader_C"))
  (set `self.LevelLoaderInstance` _returnvalue)
  (if (`self.TriggerOnStart`)
    (set `PrimitiveComponent.bGenerateOverlapEvents` false (`self.CollisionComponent`))
    (for _array_element (`self.Levels`) :!label _label
      (`/Game/Blueprints/Common/LevelLoader.EnqueueLevel` _levelloaderinstance _array_element))
    (`/Game/Blueprints/Common/LevelLoader.BeginLoad` _levelloaderinstance (`self.ShowLoadingScreen`))
    (set `self.Loaded` true)))

(event `self.ReceiveActorBeginOverlap`
  (params (OtherActor :type "Actor Object Reference"))
  (if (not (`self.TriggerOnStart`))
    (bind _asbp_player_character (cast `/Game/Blueprints/Player/BP_PlayerCharacter` OtherActor))
    (if (`self.LimitToDirection`)
      (if (> (`KismetMathLibrary.Dot_VectorVector` (`SceneComponent.GetForwardVector` (`self.Arrow`)) (`self.GetActorForwardVector` _asbp_player_character)) 0.0)
        (if (not (and (`self.TriggerOnlyOnce`) (`self.Loaded`))) :!label _label_2
          (goto _label)))
      (else
        (goto _label_2)))))

(fn `UserConstructionScript`)