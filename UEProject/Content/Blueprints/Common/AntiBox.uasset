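; AntiBox is a zone that raises the player's fear over time and resists movement toward its inner box until TriggerEvent disables it.
; While overlapped, Tick scales the cached movement modifier by squared, normalized distance to Inner, only when the player both faces and moves toward it.
; CalculateSpeed derives that factor and a 2D normal from Inner's closest collision point.
; Leaving stops the overlap effect and clears Afraid.
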(event `self.ReceiveBeginPlay`
  (bind _returnvalue (`GameplayStatics.GetActorOfClass` "/Game/Blueprints/Player/BP_PlayerCharacter.BP_PlayerCharacter_C"))
  (set `self.PlayerRef` _returnvalue)
  (set `self.DeltaDistance` (`KismetMathLibrary.FMax` (- (.x (`.BoxExtent` (`KismetSystemLibrary.GetComponentBounds` (`self.CollisionComponent`)))) (.x (`BoxComponent.BoxExtent` (`self.Inner`)))) (- (.y (`.BoxExtent` (`KismetSystemLibrary.GetComponentBounds` (`self.CollisionComponent`)))) (.y (`BoxComponent.BoxExtent` (`self.Inner`)))))))

(event `self.ReceiveTick`
  (params (DeltaSeconds :type "Float (single-precision)"))
  (bind _playerref (`self.PlayerRef`))
  (if (and (`self.InOuter`) (`self.Enabled`))
    (`/Game/Blueprints/Player/BP_PlayerCharacter.SetFearAmount` _playerref (* DeltaSeconds 0.2) true 0.0)
    (bind (_surfacenormal _speed) (`self.CalculateSpeed`))
    (if (and (< (`KismetMathLibrary.DotProduct2D` _surfacenormal (`KismetMathLibrary.Conv_VectorToVector2D` (`self.GetActorForwardVector` (`self.PlayerRef`)))) 0.0) (< (`KismetMathLibrary.DotProduct2D` _surfacenormal (`KismetMathLibrary.Normal2D` (`KismetMathLibrary.Conv_VectorToVector2D` (`Pawn.GetLastMovementInputVector` _playerref)))) 0.0))
      (`/Game/Blueprints/Player/BP_PlayerCharacter.SetMovementModifier` (`self.PlayerRef`) (* (`self.CachedSpeed`) (`KismetMathLibrary.MultiplyMultiply_FloatFloat` _speed 2.0)))
      (else
        (`/Game/Blueprints/Player/BP_PlayerCharacter.SetMovementModifier` (`self.PlayerRef`) (`self.CachedSpeed`))))))

(event `self.ReceiveActorBeginOverlap`
  (params (OtherActor :type "Actor Object Reference"))
  (if (and (== OtherActor (`self.PlayerRef`)) (`self.Enabled`))
    (set `self.InOuter` true)
    (set `self.CachedSpeed` (`/Game/Blueprints/Player/BP_PlayerCharacter.MovementModifier` (`self.PlayerRef`)))))

(event `self.ReceiveActorEndOverlap`
  (params (OtherActor :type "Actor Object Reference"))
  (if (and (== OtherActor (`self.PlayerRef`)) (`self.Enabled`))
    (set `self.InOuter` false)
    (set `/Game/Blueprints/Player/BP_PlayerCharacter.Afraid` false (`self.PlayerRef`))))

(event `/Game/Blueprints/Common/Interfaces/ITriggerable.TriggerEvent`
  (params (TriggerObject :type "/Game/Blueprints/Common/EventTrigger Object Reference"))
  (set `self.Enabled` false)
  (`PrimitiveComponent.SetCollisionEnabled` (`self.Inner`) "NoCollision")
  (`PrimitiveComponent.SetCollisionEnabled` (`self.CollisionComponent`) "NoCollision"))

(fn `CalculateSpeed`
  (returns (SurfaceNormal :type "Vector2D Structure") (Speed :type "Float (double-precision)"))
  (bind _playerref (`self.PlayerRef`))
  (bind _returnvalue (`self.K2_GetActorLocation` _playerref))
  (bind (_outpointonbody _returnvalue_2) (`PrimitiveComponent.GetClosestPointOnCollision` (`self.Inner`) _returnvalue "None"))
  (return (`KismetMathLibrary.Normal2D` (- (`KismetMathLibrary.Conv_VectorToVector2D` _returnvalue) (`KismetMathLibrary.Conv_VectorToVector2D` _outpointonbody))) (/ (- _returnvalue_2 (`CapsuleComponent.CapsuleRadius` (`Character.CapsuleComponent` _playerref))) (`self.DeltaDistance`))))

(fn `UserConstructionScript`)