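; Interactable teleporter that moves the player character to a set location after loading the levels needed there.
; On interact, it zeroes the player's gravity, queues its level list on the game instance's level loader and starts loading without a loading screen.
; After a fixed delay, rather than a load-completion callback, it teleports the player and sets gravity scale back to normal.
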(event `self.OnInteract`
  (bind _bp_game_instance (`/Game/Blueprints/Common/MacroLibrary.MGetGameInstance`))
  (bind _playercharacterref (`/Game/Blueprints/Player/BP_GameInstance.PlayerCharacterRef` _bp_game_instance))
  (bind _charactermovement (`Character.CharacterMovement` _playercharacterref))
  (set `CharacterMovementComponent.GravityScale` 0.0 _charactermovement)
  (for _array_element (`self.LoadLevels`)
    (bind _levelloaderinstance (`/Game/Blueprints/Player/BP_GameInstance.LevelLoaderInstance` _bp_game_instance))
    (`/Game/Blueprints/Common/LevelLoader.EnqueueLevel` _levelloaderinstance _array_element))
  (`/Game/Blueprints/Common/LevelLoader.BeginLoad` _levelloaderinstance false (struct :`A` 1.0) true)
  (`KismetSystemLibrary.Delay` 1.0)
  (`self.K2_SetActorLocation` _playercharacterref (`self.TeleportLocation`) false true)
  (set `CharacterMovementComponent.GravityScale` 1.0 _charactermovement))

(fn `UserConstructionScript`
  (`parent.UserConstructionScript`))