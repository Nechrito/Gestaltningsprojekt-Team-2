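; LevelStreamTrigger is a trigger actor that streams a configured list of levels, either on BeginPlay or when the player character overlaps it.
; It finds the LevelLoader actor at BeginPlay, enqueues each entry in Levels, then begins the load with an optional loading screen.
; Start-triggered instances disable overlap events on the collision component, while overlap-triggered ones can use TriggerOnlyOnce and a Loaded flag to block repeat loads.
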(event `self.ReceiveBeginPlay`
  (bind _levelloaderinstance (`self.LevelLoaderInstance`))
  (bind _returnvalue (`GameplayStatics.GetActorOfClass` "/Game/Blueprints/LevelLoader.LevelLoader_C"))
  (set `self.LevelLoaderInstance` _returnvalue)
  (if (`self.TriggerOnStart`)
    (set `PrimitiveComponent.bGenerateOverlapEvents` false (`self.CollisionComponent`))
    (for _array_element (`self.Levels`) :!label _label
      (`/Game/Blueprints/LevelLoader.EnqueueLevel` _levelloaderinstance _array_element))
    (`/Game/Blueprints/LevelLoader.BeginLoad` _levelloaderinstance (`self.ShowLoadingScreen`))
    (set `self.Loaded` true)))

(event `self.ReceiveActorBeginOverlap`
  (params (OtherActor :type "Actor Object Reference"))
  (if (not (`self.TriggerOnStart`))
    (cast `/Game/Blueprints/Player/BP_PlayerCharacter` OtherActor)
    (if (not (and (`self.TriggerOnlyOnce`) (`self.Loaded`)))
      (goto _label))))

(event `Enqueue`)

(fn `UserConstructionScript`)