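; Water controller that fits an underwater post-process effect and a surface collision box to a physics volume.
; On BeginPlay it reads the volume's brush bounds to size and place PostProcessBounds, lowered at the top by PostProcessDepth.
; SurfaceCollision becomes a thin slab near the water top, set by SurfaceThickness and SurfaceOffset.
; The post process is made bounded and given the underwater settings; nothing updates afterwards.
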(event `self.ReceiveBeginPlay`
  (bind _surfacecollision (`self.SurfaceCollision`))
  (bind _postprocess (`self.PostProcess`))
  (bind _returnvalue (* (`self.SurfaceThickness`) 0.5))
  (bind _returnvalue_2 (* (`self.PostProcessDepth`) 0.5))
  (bind (_origin _boxextent) (`KismetSystemLibrary.GetComponentBounds` (`Brush.BrushComponent` (`self.PhysicsVolume`))))
  (bind _x (.x _boxextent))
  (bind _y (.y _boxextent))
  (bind _z (.z _boxextent))
  (`SceneComponent.K2_SetWorldLocation` (`self.PostProcessBounds`) (+ _origin (`KismetMathLibrary.MakeVector` 0.0 0.0 (* _returnvalue_2 -1.0))) false true)
  (`BoxComponent.SetBoxExtent` _surfacecollision (`KismetMathLibrary.MakeVector` _x _y _returnvalue) true)
  (`SceneComponent.K2_SetRelativeLocation` _surfacecollision (`KismetMathLibrary.MakeVector` 0.0 0.0 (+ (- (+ _z _returnvalue_2) _returnvalue) (`self.SurfaceOffset`))) false true)
  (`BoxComponent.SetBoxExtent` (`self.PostProcessBounds`) (`KismetMathLibrary.MakeVector` _x _y (- _z _returnvalue_2)) true)
  (set `PostProcessComponent.bUnbound` false _postprocess)
  (set `PostProcessComponent.Settings` (`self.UnderwaterPostProcessing`) _postprocess))

(fn `NewFunction_0`)

(fn `UserConstructionScript`)