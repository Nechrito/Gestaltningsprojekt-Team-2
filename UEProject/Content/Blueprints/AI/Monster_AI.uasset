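; Monster AI controller that runs the monster's behavior tree and feeds it patrol and perception data through the blackboard.
; On begin play it starts Monster_BT and copies the possessed Monster's patrol path looping and wait time, plus an initial direction, to the blackboard.
; Perception updates treat Noise-tagged stimuli as investigation targets with a location, and all other stimuli as whether the player is visible.
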(event `self.ReceiveBeginPlay`
  (bind _returnvalue (`AIBlueprintHelperLibrary.GetBlackboard` null))
  (`self.RunBehaviorTree` "/Game/Blueprints/AI/Monster_BT.Monster_BT")
  (bind _asmonster (cast `/Game/Blueprints/AI/Monster` (`self.K2_GetPawn`)))
  (bind _output_get (set `self.MyPawn` _asmonster))
  (`BlackboardComponent.SetValueAsBool` (`AIBlueprintHelperLibrary.GetBlackboard` null) "PathLooping" (`/Game/Blueprints/AI/PatrolPath.IsLooping` (`/Game/Blueprints/AI/Monster.PatrolPath` _output_get)))
  (`BlackboardComponent.SetValueAsInt` _returnvalue "Direction" 1)
  (`BlackboardComponent.SetValueAsFloat` _returnvalue "WaitTime" (`/Game/Blueprints/AI/PatrolPath.WaitTime` (`/Game/Blueprints/AI/Monster.PatrolPath` (`self.MyPawn`)))))

(event `self.AIPerception.OnPerceptionUpdated`
  (params (UpdatedActors :type "Array of Actor Object Reference (by ref)"))
  ;[1 1 1] Comment
  (for _array_element UpdatedActors
    (bind _info (`AIPerceptionComponent.GetActorsPerception` (`self.AIPerception`) _array_element))
    (for _array_element_2 (`.LastSensedStimuli` (break `ActorPerceptionBlueprintInfo` _info))
      (bind (_age _expirationage _strength _stimuluslocation _receiverlocation _tag _bsuccessfullysensed) (break `AIStimulus` _array_element_2))
      (if (== _tag "Noise")
        (`BlackboardComponent.SetValueAsBool` (`AIBlueprintHelperLibrary.GetBlackboard` null) "IsInvestigating" _bsuccessfullysensed)
        (`BlackboardComponent.SetValueAsVector` (`AIBlueprintHelperLibrary.GetBlackboard` null) "TargetLocation" _stimuluslocation)
        (else
          (`BlackboardComponent.SetValueAsBool` (`AIBlueprintHelperLibrary.GetBlackboard` null) "CanSeePlayer" _bsuccessfullysensed))))))

(fn `UserConstructionScript`)