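; Stealth player Blueprint that works out how visible the player is from lighting each tick and prints it as a percentage.
; It traces toward the first directional light found at BeginPlay, setting visibility to full on a hit and zero otherwise.
; It then adds the brightness of every entry in its Lights array, with no distance or occlusion test here, and clamps the total.
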(event `self.ReceiveBeginPlay`
  (bind _outactors (`GameplayStatics.GetAllActorsOfClass` "/Script/Engine.DirectionalLight"))
  (set `self.Sun` (`|GetArrayItem` _outactors)))

(event `self.ReceiveTick`
  (params (DeltaSeconds :type "Float (single-precision)"))
  (`self.CheckSunlight`)
  (`self.CheckPointLights`)
  (`KismetSystemLibrary.PrintText` (`|FormatText` "You're {x}% visible" (* (`self.Visibility`) 100.0)) true false (struct :`G` 0.66 :`B` 1.0 :`A` 1.0) 0.0))

(fn `CheckPointLights`
  (for _array_element (`self.Lights`)
    (set `self.Visibility` (+ (`/Game/Blueprints/AI/Stealth/StealthLight.Brightness` _array_element) (`self.Visibility`))))
  (set `self.Visibility` (`KismetMathLibrary.FClamp` (`self.Visibility`) 0.0 1.0)))

(fn `CheckSunlight`
  (bind _returnvalue (`self.K2_GetActorLocation`))
  (bind (_outhit _returnvalue_2) (`KismetSystemLibrary.LineTraceSingle` _returnvalue (+ _returnvalue (* (`self.GetActorForwardVector` (`self.Sun`)) -100000)) "TraceTypeQuery1"))
  (if _returnvalue_2
    (set `self.Visibility` 1.0)
    (else
      (set `self.Visibility` 0.0))))

(fn `UserConstructionScript`
  (`parent.UserConstructionScript`))