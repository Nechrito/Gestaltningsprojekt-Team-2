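; ForestWater is a Level 2 water hazard that periodically damages the player while they are inside its box volume.
; BeginPlay caches the player and sets the actor tick interval to DamageTick, so Tick applies damage when DamageEnabled and Overlapping are true.
; Two NoCollision volumes set a shared NoDamage flag that suppresses damage and sounds.
; Entering or leaving the box plays sounds at the player's feet, throttled by a one-second lockout.
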(event `self.ReceiveBeginPlay`
  (bind _bp_player_character (`/Game/Blueprints/Common/MacroLibrary.MGetPlayerCharacter`))
  (set `self.PlayerCharacterRef` _bp_player_character)
  (`self.SetActorTickInterval` (`self.DamageTick`))
  (`self.SetActorTickEnabled` true))

(event `self.ReceiveTick`
  (params (DeltaSeconds :type "Float (single-precision)"))
  (if (and (`self.DamageEnabled`) (not (`self.NoDamage`)) (`self.Overlapping`))
    (`GameplayStatics.ApplyDamage` (`self.PlayerCharacterRef`) (`self.DamageAmount`) null self "/Game/Blueprints/Player/PlayerGenericDamage.PlayerGenericDamage_C")))

(event `self.NoCollision.OnComponentBeginOverlap`
  (params (OverlappedComponent :type "PrimitiveComponent Object Reference") (OtherActor :type "Actor Object Reference") (OtherComp :type "PrimitiveComponent Object Reference") (OtherBodyIndex :type Integer) (bFromSweep :type Boolean) (SweepResult :type "HitResult Structure (by ref)"))
  (if (== OtherActor (`self.PlayerCharacterRef`))
    (set `self.NoDamage` true)))

(event `self.NoCollision.OnComponentEndOverlap`
  (params (OverlappedComponent :type "PrimitiveComponent Object Reference") (OtherActor :type "Actor Object Reference") (OtherComp :type "PrimitiveComponent Object Reference") (OtherBodyIndex :type Integer))
  (if (== OtherActor (`self.PlayerCharacterRef`))
    (set `self.NoDamage` false)))

(event `self.NoCollision2.OnComponentBeginOverlap`
  (params (OverlappedComponent :type "PrimitiveComponent Object Reference") (OtherActor :type "Actor Object Reference") (OtherComp :type "PrimitiveComponent Object Reference") (OtherBodyIndex :type Integer) (bFromSweep :type Boolean) (SweepResult :type "HitResult Structure (by ref)"))
  (if (== OtherActor (`self.PlayerCharacterRef`))
    (set `self.NoDamage` true)))

(event `self.NoCollision2.OnComponentEndOverlap`
  (params (OverlappedComponent :type "PrimitiveComponent Object Reference") (OtherActor :type "Actor Object Reference") (OtherComp :type "PrimitiveComponent Object Reference") (OtherBodyIndex :type Integer))
  (if (== OtherActor (`self.PlayerCharacterRef`))
    (set `self.NoDamage` false)))

(event `self.BoxCollision.OnComponentBeginOverlap`
  (params (OverlappedComponent :type "PrimitiveComponent Object Reference") (OtherActor :type "Actor Object Reference") (OtherComp :type "PrimitiveComponent Object Reference") (OtherBodyIndex :type Integer) (bFromSweep :type Boolean) (SweepResult :type "HitResult Structure (by ref)"))
  (bind _playercharacterref (`self.PlayerCharacterRef`))
  (if (== OtherActor (`self.PlayerCharacterRef`))
    (set `self.Overlapping` true)
    (if (and (not (`self.NoDamage`)) (not (`self.SoundIsPlaying`)))
      (`/Game/Blueprints/Player/BP_GameInstance.PlayCharacterSound` (`/Game/Blueprints/Player/BP_PlayerCharacter.GameInstanceRef` _playercharacterref) (`/Game/Blueprints/Player/BP_PlayerCharacter.Feet` _playercharacterref) "NewEnumerator30" 1.0 "NewEnumerator8")
      (set `self.SoundIsPlaying` true :!label _label)
      (`KismetSystemLibrary.Delay` 1.0)
      (set `self.SoundIsPlaying` false))))

(event `self.BoxCollision.OnComponentEndOverlap`
  (params (OverlappedComponent :type "PrimitiveComponent Object Reference") (OtherActor :type "Actor Object Reference") (OtherComp :type "PrimitiveComponent Object Reference") (OtherBodyIndex :type Integer))
  (bind _playercharacterref (`self.PlayerCharacterRef`))
  (if (== OtherActor (`self.PlayerCharacterRef`))
    (set `self.Overlapping` false)
    (if (and (not (`self.NoDamage`)) (not (`self.SoundIsPlaying`)))
      (`/Game/Blueprints/Player/BP_GameInstance.PlayCharacterSound` (`/Game/Blueprints/Player/BP_PlayerCharacter.GameInstanceRef` _playercharacterref) (`/Game/Blueprints/Player/BP_PlayerCharacter.Feet` _playercharacterref) "NewEnumerator24" 1.0 "NewEnumerator8")
      (goto _label))))

(fn `UserConstructionScript`)