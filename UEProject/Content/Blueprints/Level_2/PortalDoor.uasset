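; A portal door actor that opens once the player has placed held symbols and all required global flags are set, then teleports the player.
; Tick shows or hides the wall and placed symbols by camera facing and line side, and scales the open portal by view angle.
; Symbols auto-place when a triggered player stands still facing the door.
; Entering the open, visible portal loads configured levels behind a loading screen and relocates the player.
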(event `self.ReceiveBeginPlay`
  (bind _linelength (`self.LineLength`))
  (bind _returnvalue (`KismetMathLibrary.Conv_VectorToVector2D` (`self.GetActorRightVector`)))
  (bind _returnvalue_2 (`KismetMathLibrary.Conv_VectorToVector2D` (- (`SceneComponent.K2_GetComponentLocation` (`self.Center`)) (* (`self.GetActorForwardVector`) 100.0))))
  (bind _bp_game_instance (`/Game/Blueprints/Common/MacroLibrary.MGetGameInstance`))
  (set `self.GameInstanceRef` _bp_game_instance)
  (bind _bp_player_character (`/Game/Blueprints/Common/MacroLibrary.MGetPlayerCharacter`))
  (set `self.PlayerCharacterRef` _bp_player_character)
  (`self.SetActorTickEnabled` true)
  (`SceneComponent.SetVisibility` (`self.Portal`) false false)
  (bind _output_get (set `self.LineA` (+ (* _returnvalue (* _linelength -1.0)) _returnvalue_2)))
  (bind _output_get_2 (set `self.LineB` (+ (* _returnvalue _linelength) _returnvalue_2)))
  (set `self.Line` (- _output_get_2 _output_get))
  (`TimelineComponent.SetPlayRate` (`self.Timeline_0`) (`self.OpenSpeed`)))

(event `self.ReceiveTick`
  (params (DeltaSeconds :type "Float (single-precision)"))
  (bind _wall (`self.Wall`))
  (bind _waittimer (`self.WaitTimer`))
  (bind _visible (`self.Visible`))
  (bind _playercamera (`/Game/Blueprints/Player/BP_PlayerCharacter.PlayerCamera` (`self.PlayerCharacterRef`)))
  (bind _returnvalue (`KismetMathLibrary.DotProduct2D` (`KismetMathLibrary.Normal2D` (`KismetMathLibrary.Conv_VectorToVector2D` (`SceneComponent.GetForwardVector` _playercamera))) (`KismetMathLibrary.Conv_VectorToVector2D` (`self.GetActorForwardVector`))))
  (`|ExecutionSequence`
    (:`then_0`
      (if (`self.Open`)
        (`SceneComponent.SetRelativeScale3D` (`self.Portal`) (`KismetMathLibrary.MakeVector` (+ (* (- (`KismetMathLibrary.Abs` (`KismetMathLibrary.FClamp` _returnvalue -1.0 -0.5)) 0.5) 1.9) 0.05) 1.0 1.0)))
      (if (or (> _returnvalue 0.75) (< (`KismetMathLibrary.CrossProduct2D` (- (`KismetMathLibrary.Conv_VectorToVector2D` (`SceneComponent.K2_GetComponentLocation` _playercamera)) (`self.LineA`)) (`self.Line`)) 0.0))
        (if _visible
          (`SceneComponent.SetVisibility` _wall false true)
          (set `self.Visible` false)
          (for _array_element (`self.PlacedSymbols`) :!label _label
            (`/Game/Blueprints/Level_2/Symbol.SetVisibility` _array_element (`self.Visible`))))
        (elif (not _visible)
          (`SceneComponent.SetVisibility` _wall true true)
          (set `self.Visible` true)
          (goto _label))))
    (:`then_1`
      (if (`self.Waiting`)
        (if (and (< _returnvalue -0.7) (`KismetMathLibrary.Vector_IsNearlyZero` (`self.GetVelocity` (`self.PlayerCharacterRef`)) 0.1))
          (set `self.WaitTimer` (+ _waittimer DeltaSeconds))
          (if (> _waittimer 0.25)
            (set `self.Waiting` false)
            (set `self.WaitTimer` 0.0)
            (`self.PlaceSymbol`)))))))

(event `OpenPortal`
  (bind _door (`self.Door`))
  (`SceneComponent.SetVisibility` (`self.Portal`) true true)
  (set `self.Open` true)
  (`/Game/Blueprints/Player/BP_GameInstance.PlayLocalizedSound` (`self.GameInstanceRef`) (`SceneComponent.K2_GetComponentLocation` (`self.Center`)) "NewEnumerator8" 1.0 "NewEnumerator8")
  (bind (_direction _rotation _translation) (`Timeline|Timeline_0`)
    (:`Update`
      (`SceneComponent.K2_SetRelativeRotation` _door (`KismetMathLibrary.RLerp` (struct) (struct :`Yaw` -100.0) (`KismetMathLibrary.MultiplyMultiply_FloatFloat` _rotation 3.0)) false false)
      (`SceneComponent.K2_SetRelativeLocation` _door (`KismetMathLibrary.VLerp` (0.0 0.0 0.0) (-100.0 20.0 0.0) _translation) false true))
    (:`Finished`
      (`SceneComponent.SetVisibility` (`self.Door`) false true))))

(event `self.PortalTrigger.OnComponentBeginOverlap`
  (params (OverlappedComponent :type "PrimitiveComponent Object Reference") (OtherActor :type "Actor Object Reference") (OtherComp :type "PrimitiveComponent Object Reference") (OtherBodyIndex :type Integer) (bFromSweep :type Boolean) (SweepResult :type "HitResult Structure (by ref)"))
  (if (and (== OtherActor (`self.PlayerCharacterRef`)) (`self.Open`) (`self.Visible`))
    (`/Game/Blueprints/Player/BP_GameInstance.PlayLocalizedSound` (`self.GameInstanceRef`) (`SceneComponent.K2_GetComponentLocation` (`self.Center`)) "NewEnumerator8" 1.0 "NewEnumerator8")
    (`self.Teleport`)))

(event `self.SymbolTrigger.OnComponentBeginOverlap`
  (params (OverlappedComponent :type "PrimitiveComponent Object Reference") (OtherActor :type "Actor Object Reference") (OtherComp :type "PrimitiveComponent Object Reference") (OtherBodyIndex :type Integer) (bFromSweep :type Boolean) (SweepResult :type "HitResult Structure (by ref)"))
  (bind _playercharacterref (`self.PlayerCharacterRef`))
  (if (and (== OtherActor _playercharacterref) (not (`self.Open`)) (`self.Visible`) (`/Game/Blueprints/Player/BP_PlayerCharacter.HoldingSymbol` _playercharacterref))
    (set `self.Waiting` true)))

(event `PlaceSymbol`
  (bind _playercharacterref (`self.PlayerCharacterRef`))
  (bind _heldsymbol (`/Game/Blueprints/Player/BP_PlayerCharacter.HeldSymbol` (`self.PlayerCharacterRef`)))
  (`KismetArrayLibrary.Array_Add` (`self.PlacedSymbols`) _heldsymbol)
  (switch `int` (`/Game/Blueprints/Level_2/Symbol.Placement` _heldsymbol)
    (:`1`
      (`/Game/Blueprints/Player/BP_PlayerCharacter.PlaceSymbol` _playercharacterref (`self.SymbolNode1`)))
    (:`2`
      (`/Game/Blueprints/Player/BP_PlayerCharacter.PlaceSymbol` _playercharacterref (`self.SymbolNode2`)))
    (:`3`
      (`/Game/Blueprints/Player/BP_PlayerCharacter.PlaceSymbol` _playercharacterref (`self.SymbolNode3`)))
    (:`4`
      (`/Game/Blueprints/Player/BP_PlayerCharacter.PlaceSymbol` _playercharacterref (`self.SymbolNode4`)))
    (:`5`
      (`/Game/Blueprints/Player/BP_PlayerCharacter.PlaceSymbol` _playercharacterref (`self.SymbolNode5`))))
  (`KismetSystemLibrary.Delay` 4.5)
  (bind _exists (`self.CheckFlags`))
  (if _exists
    (`self.OpenPortal`)))

(event `Teleport`
  (bind _playercharacterref (`self.PlayerCharacterRef`))
  (bind _levelloaderinstance (`/Game/Blueprints/Player/BP_GameInstance.LevelLoaderInstance` (`self.GameInstanceRef`)))
  (bind _charactermovement (`Character.CharacterMovement` _playercharacterref))
  (set `CharacterMovementComponent.GravityScale` 0.0 _charactermovement)
  (for _array_element (`self.LoadLevels`)
    (`/Game/Blueprints/Common/LevelLoader.EnqueueLevel` _levelloaderinstance _array_element))
  (`/Game/Blueprints/Common/LevelLoader.BeginLoad` _levelloaderinstance true (struct :`R` 1.0 :`G` 1.0 :`B` 1.0 :`A` 1.0) false)
  (`KismetSystemLibrary.Delay` 1.0)
  (`self.K2_SetActorLocation` _playercharacterref (`self.TeleportLocation`) false true)
  (`Controller.SetControlRotation` (`/Game/Blueprints/Player/BP_PlayerCharacter.PlayerControllerRef` (`self.PlayerCharacterRef`)) (`KismetMathLibrary.Conv_VectorToRotator` (`self.TeleportDirection`)))
  (set `CharacterMovementComponent.GravityScale` 1.0 _charactermovement))

(fn `CheckFlags`
  (returns (Exists :type Boolean))
  (for _array_element (`self.GlobalFlags`)
    (bind _flagexists (`/Game/Blueprints/Player/BP_GameInstance.CheckGlobalFlag` (`self.GameInstanceRef`) _array_element))
    (if (not _flagexists)
      (return false)))
  (return true))

(fn `UserConstructionScript`)