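; Level 2 interactable symbol pickup that the player grabs with the left hand, playing a localized sound.
; It disables itself when an overlapping player already holds a symbol, and its trigger event blocks further use and sets a global flag.
; BeginPlay registers it for saving, caches a Symbol2DCapture actor and creates a dynamic glowing material.
; Save and load persist its transform and disabled state.
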(event `self.ReceiveBeginPlay`
  (`parent.ReceiveBeginPlay`)
  (`/Game/Blueprints/Common/MacroLibrary.MRegisterSaveable`)
  (bind _bp_game_instance (`/Game/Blueprints/Common/MacroLibrary.MGetGameInstance`))
  (set `self.GameInstanceRef` _bp_game_instance)
  (bind _outactors (`GameplayStatics.GetAllActorsOfClass` "/Game/Blueprints/Level_2/Symbol2DCapture.Symbol2DCapture_C"))
  (set `self.SceneCaptureRef` (`|GetArrayItem` _outactors))
  (bind _returnvalue (`PrimitiveComponent.CreateDynamicMaterialInstance` (`self.StaticMesh`) 0 "/Game/Assets/Materials/Level_2/Glowing_Symbol.Glowing_Symbol" "None"))
  (set `self.MaterialInstance` _returnvalue))

(event `self.ReceiveTick`
  (params (DeltaSeconds :type "Float (single-precision)"))
  (`parent.ReceiveTick` DeltaSeconds))

(event `/Game/Blueprints/Common/Interfaces/ISaveable.LoadState`
  (params (Data :type "/Game/Blueprints/Common/Structs/SaveableData Structure"))
  (bind (_name _transform _isactivated) (break `/Game/Blueprints/Common/Structs/SaveableData` Data))
  (set `self.Disabled` (not _isactivated))
  (`SceneComponent.K2_SetWorldTransform` (`self.RootComponent`) _transform false true))

(event `self.OnInteract`
  (bind _returnvalue (`self.K2_GetActorLocation`))
  (bind _gameinstanceref (`self.GameInstanceRef`))
  (`/Game/Blueprints/Player/BP_PlayerCharacter.GrabObjectLeftHand` (`/Game/Blueprints/Player/BP_GameInstance.PlayerCharacterRef` _gameinstanceref) _returnvalue self)
  (`/Game/Blueprints/Player/BP_GameInstance.PlayLocalizedSound` _gameinstanceref _returnvalue "NewEnumerator18" 1.0 "NewEnumerator8"))

(event `/Game/Blueprints/Common/Interfaces/ITriggerable.TriggerEvent`
  (params (TriggerObject :type "/Game/Blueprints/Common/EventTrigger Object Reference"))
  (set `self.CanUse` false)
  (`/Game/Blueprints/Player/BP_GameInstance.SetGlobalFlag` (`self.GameInstanceRef`) (`self.GlobalFlag`)))

(event `self.ReceiveActorBeginOverlap`
  (params (OtherActor :type "Actor Object Reference"))
  (bind _asbp_player_character (cast `/Game/Blueprints/Player/BP_PlayerCharacter` OtherActor))
  (if (`/Game/Blueprints/Player/BP_PlayerCharacter.HoldingSymbol` _asbp_player_character)
    (set `self.Disabled` true)
    (else
      (set `self.Disabled` false)))
  (`parent.ReceiveActorBeginOverlap` OtherActor))

(event `SetVisibility`
  (params (Visible :type Boolean :default true))
  (`SceneComponent.SetVisibility` (`self.StaticMesh`) Visible false))

(fn `SaveState`
  (returns (Data :type "/Game/Blueprints/Common/Structs/SaveableData Structure"))
  (return (make `/Game/Blueprints/Common/Structs/SaveableData` (`KismetStringLibrary.Conv_StringToName` (`KismetSystemLibrary.GetObjectName` self)) (`SceneComponent.K2_GetComponentToWorld` (`self.RootComponent`)) (not (`self.Disabled`)))))

(fn `UserConstructionScript`
  (`parent.UserConstructionScript`))