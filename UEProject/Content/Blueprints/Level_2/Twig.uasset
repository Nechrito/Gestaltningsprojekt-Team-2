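; Twig is a Level 2 one-shot noise trigger that gives away the player on stepping into it.
; The first overlap by an actor whose class is exactly BP_PlayerCharacter sets a Triggered flag, so it never fires again.
; It then plays a sound at its Sphere through the game instance's PlayCharacterSound and reports a tagged AI noise event at its location, with itself as instigator.
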(event `self.ReceiveActorBeginOverlap`
  (params (OtherActor :type "Actor Object Reference"))
  (if (and (not (`self.Triggered`)) (== (`GameplayStatics.GetObjectClass` OtherActor) "/Game/Blueprints/Player/BP_PlayerCharacter.BP_PlayerCharacter_C"))
    (set `self.Triggered` true)
    (bind _bp_game_instance (`/Game/Blueprints/Common/MacroLibrary.MGetGameInstance`))
    (`/Game/Blueprints/Player/BP_GameInstance.PlayCharacterSound` _bp_game_instance (`self.Sphere`) "NewEnumerator7" 1.0 "NewEnumerator1")
    (`AISense_Hearing.ReportNoiseEvent` (`self.K2_GetActorLocation`) 0.75 self 0.0 "Noise")))

(fn `UserConstructionScript`
  (`parent.UserConstructionScript`))