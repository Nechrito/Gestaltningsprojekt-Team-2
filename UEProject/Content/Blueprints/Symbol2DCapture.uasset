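; Scene capture actor that isolates a Symbol mesh and controls the fade of the HUD's symbol image.
; On BeginPlay it limits the capture to that mesh, waits a second, then caches the Hud_Widget and its SymbolImage dynamic material.
; Show swaps the mesh, makes the image visible and plays a timeline driving the material's Opacity.
; Hide reverses that timeline, collapsing the image when it finishes.
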(event `self.ReceiveBeginPlay`
  (`SceneCaptureComponent.ShowOnlyComponent` (`self.CaptureComponent2D`) (`self.Symbol`))
  (`KismetSystemLibrary.Delay` 1.0)
  (bind _foundwidgets (`WidgetBlueprintLibrary.GetAllWidgetsOfClass` "/Game/Blueprints/Widgets/Hud_Widget.Hud_Widget_C"))
  (bind _output_get (set `self.HudWidgetRef` (`|GetArrayItem` _foundwidgets)))
  (bind _returnvalue (`Image.GetDynamicMaterial` (`/Game/Blueprints/Widgets/Hud_Widget.SymbolImage` _output_get)))
  (set `self.UIMaterial` _returnvalue))

(event `Show`
  (params (Mesh :type "StaticMesh Object Reference"))
  (`StaticMeshComponent.SetStaticMesh` (`self.Symbol`) Mesh)
  (`Widget.SetVisibility` (`/Game/Blueprints/Widgets/Hud_Widget.SymbolImage` (`self.HudWidgetRef`)) "Visible")
  (bind (_direction _float) (`Timeline|Timeline_0` :!via `PlayFromStart` :!label _label)
    (:`Update`
      (`MaterialInstanceDynamic.SetScalarParameterValue` (`self.UIMaterial`) "Opacity" _float))
    (:`Finished`
      (if (`|EnumEquality` _direction "Backward")
        (`Widget.SetVisibility` (`/Game/Blueprints/Widgets/Hud_Widget.SymbolImage` (`self.HudWidgetRef`)) "Collapsed")))))

(event `Hide`
  (goto _label :!via `ReverseFromEnd`))

(fn `UserConstructionScript`)