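; Watergun is a saveable, physics-simulated weapon pickup that the player grabs into the right hand on interact.
; Triggering plays a localized sound and a timeline that drives particle spawn and intensity, blocking refire until it finishes.
; Each particle collision applies radial damage at the impact point.
; After BeginPlay, Tick waits for the mesh to come to rest, then repositions the interact billboard, enables use and checks overlaps.
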(event `self.ReceiveBeginPlay`
  (`parent.ReceiveBeginPlay`)
  (`/Game/Blueprints/MacroLibrary.MRegisterSaveable`)
  (bind _bp_game_instance (`/Game/Blueprints/MacroLibrary.MGetGameInstance`))
  (set `self.GameInstanceRef` _bp_game_instance)
  (`KismetSystemLibrary.Delay` 0.2)
  (set `self.InMotion` true))

(event `self.ReceiveTick`
  (params (DeltaSeconds :type "Float (single-precision)"))
  (`parent.ReceiveTick` DeltaSeconds)
  (if (`self.InMotion`)
    (bind _returnvalue (`PrimitiveComponent.GetPhysicsLinearVelocity` (`self.StaticMesh`) "None"))
    (if (and (== _returnvalue (0.0 0.0 0.0) :`ErrorTolerance` 0.01) (== (`PrimitiveComponent.GetPhysicsAngularVelocityInRadians` (`self.StaticMesh`) "None") (0.0 0.0 0.0) :`ErrorTolerance` 0.001))
      (`self.OnPhysicsEnd`))))

(event `/Game/Blueprints/ISaveable.LoadState`
  (params (Data :type "/Game/Blueprints/SaveableData Structure"))
  (`SceneComponent.K2_SetWorldTransform` (`self.RootComponent`) (`.Transform_17_26866086461CE03CEEE979AE8AEB219A` (break `/Game/Blueprints/SaveableData` Data)) false true))

(event `self.OnInteract`
  (bind _asbp_player_character (cast `/Game/Blueprints/Player/BP_PlayerCharacter` (`GameplayStatics.GetPlayerCharacter` 0)))
  (`/Game/Blueprints/Player/BP_PlayerCharacter.GrabObjectRightHand` :`self` _asbp_player_character :`Location` (`self.K2_GetActorLocation`) :`Object` self :`IsWeapon` true)
  (`/Game/Blueprints/Player/BP_GameInstance.PlayLocalizedSound` (`self.GameInstanceRef`) (`self.K2_GetActorLocation`) "NewEnumerator22" 1.0 "NewEnumerator2"))

(event `/Game/Blueprints/ITriggerable.TriggerEvent`
  (params (TriggerObject :type "/Game/Blueprints/EventTrigger Object Reference"))
  (bind _instanceparameters (`ParticleSystemComponent.InstanceParameters` (`self.ParticleSystem`)))
  (if (not (`self.Firing`))
    (set `self.Firing` true)
    (`/Game/Blueprints/Player/BP_GameInstance.PlayLocalizedSound` (`self.GameInstanceRef`) (`self.K2_GetActorLocation`) "NewEnumerator24" 1.0 "NewEnumerator2")
    (bind (_direction _spawn _intensity) (`Timeline|FireTimeline` :!via `PlayFromStart`)
      (:`Update`
        (setmembers `ParticleSysParam` :`StructRef` (`|GetArrayItem` _instanceparameters) :`Scalar` _spawn)
        (setmembers `ParticleSysParam` :`StructRef` (`|GetArrayItem` _instanceparameters 1) :`Scalar` _intensity))
      (:`Finished`
        (set `self.Firing` false)))))

(event `self.ParticleSystem.OnParticleCollide`
  (params (EventName :type Name) (EmitterTime :type "Float (single-precision)") (ParticleTime :type Integer) (Location :type "Vector Structure") (Velocity :type "Vector Structure") (Direction :type "Vector Structure") (Normal :type "Vector Structure") (BoneName :type Name) (PhysMat :type "PhysicalMaterial Object Reference"))
  (`GameplayStatics.ApplyRadialDamage` :`BaseDamage` (`self.DamagePerHit`) :`Origin` Location :`DamageRadius` (`self.DamageRadius`) :`DamageCauser` null :`InstigatedByController` null))

(fn `OnPhysicsEnd`
  ;[1 1 1] Resets interact symbol offset after physics simulation
  (`SceneComponent.K2_SetWorldLocationAndRotation` :`self` (`self.Billboard`) :`NewLocation` (+ (`SceneComponent.K2_GetComponentLocation` (`self.StaticMesh`)) (`self.InteractOffset`)))
  (set `self.InMotion` false)
  (set `self.CanUse` true)
  (`self.CheckOverlap`))

(fn `SaveState`
  (returns (Data :type "/Game/Blueprints/SaveableData Structure"))
  (return (make `/Game/Blueprints/SaveableData` (`KismetStringLibrary.Conv_StringToName` (`KismetSystemLibrary.GetObjectName` self)) (`SceneComponent.K2_GetComponentToWorld` (`self.RootComponent`)))))

(fn `UserConstructionScript`
  (`parent.UserConstructionScript`))