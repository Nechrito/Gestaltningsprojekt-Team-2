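; Saveable water gun weapon that the player picks up through interaction and fires as a particle jet.
; Trigger events start or cut short a timeline that drives the jet's spawn and intensity, with localized sounds.
; Particle collisions apply full radial damage at the hit point, ignoring the player.
; Tick watches for the physics mesh to come to rest, then repositions the interact billboard and re-enables use.
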(event `self.ReceiveBeginPlay`
  (`parent.ReceiveBeginPlay`)
  (`/Game/Blueprints/Common/MacroLibrary.MRegisterSaveable`)
  (bind _bp_game_instance (`/Game/Blueprints/Common/MacroLibrary.MGetGameInstance`))
  (set `self.GameInstanceRef` _bp_game_instance)
  (`KismetSystemLibrary.Delay` 0.2)
  (set `self.InMotion` true))

(event `self.ReceiveTick`
  (params (DeltaSeconds :type "Float (single-precision)"))
  (`parent.ReceiveTick` DeltaSeconds)
  (if (`self.InMotion`)
    (bind _returnvalue (`PrimitiveComponent.GetPhysicsLinearVelocity` (`self.StaticMesh`) "None"))
    (if (and (== _returnvalue (0.0 0.0 0.0) :`ErrorTolerance` 0.01) (== (`PrimitiveComponent.GetPhysicsAngularVelocityInRadians` (`self.StaticMesh`) "None") (0.0 0.0 0.0) :`ErrorTolerance` 0.001))
      (`self.OnPhysicsEnd`))))

(event `/Game/Blueprints/Common/Interfaces/ISaveable.LoadState`
  (params (Data :type "/Game/Blueprints/Common/Structs/SaveableData Structure"))
  (`SceneComponent.K2_SetWorldTransform` (`self.RootComponent`) (`.Transform_17_26866086461CE03CEEE979AE8AEB219A` (break `/Game/Blueprints/Common/Structs/SaveableData` Data)) false true))

(event `self.OnInteract`
  (bind _asbp_player_character (cast `/Game/Blueprints/Player/BP_PlayerCharacter` (`GameplayStatics.GetPlayerCharacter` 0)))
  (`/Game/Blueprints/Player/BP_PlayerCharacter.GrabWeapon` _asbp_player_character (`self.K2_GetActorLocation`) (`self.K2_GetActorRotation`) self (`self.StaticMesh`))
  (`/Game/Blueprints/Player/BP_GameInstance.PlayLocalizedSound` (`self.GameInstanceRef`) (`SceneComponent.K2_GetComponentLocation` (`self.StaticMesh`)) "NewEnumerator22" 1.0 "NewEnumerator8"))

(event `/Game/Blueprints/Common/Interfaces/ITriggerable.TriggerEvent`
  (params (TriggerObject :type "/Game/Blueprints/Common/EventTrigger Object Reference"))
  (bind _particlesystem (`self.ParticleSystem`))
  (bind _returnvalue (`SceneComponent.K2_GetComponentLocation` (`self.StaticMesh`)))
  (if (`self.Firing`)
    (set `self.Firing` false)
    (bind (_direction _spawn _intensity) (`Timeline|FireTimeline` :`NewTime` 1.95 :!via `SetNewTime` :!label _label)
      (:`Update`
        (`FXSystemComponent.SetFloatParameter` _particlesystem "Spawn" _spawn)
        (`FXSystemComponent.SetFloatParameter` _particlesystem "JetIntensity" _intensity))
      (:`Finished`
        (set `self.ParticleActive` false)
        (`KismetSystemLibrary.PrintString` "End shoot!")
        (`/Game/Blueprints/Player/BP_GameInstance.PlayLocalizedSound` (`self.GameInstanceRef`) _returnvalue "NewEnumerator23" 1.0 "NewEnumerator8")))
    (elif (not (`self.ParticleActive`))
      (set `self.ParticleActive` true)
      (set `self.Firing` true)
      (`KismetSystemLibrary.PrintString` "Shoot!")
      (`/Game/Blueprints/Player/BP_GameInstance.PlayLocalizedSound` (`self.GameInstanceRef`) _returnvalue "NewEnumerator24" 1.0 "NewEnumerator8")
      (goto _label :!via `PlayFromStart`))))

(event `self.ParticleSystem.OnParticleCollide`
  (params (EventName :type Name) (EmitterTime :type "Float (single-precision)") (ParticleTime :type Integer) (Location :type "Vector Structure") (Velocity :type "Vector Structure") (Direction :type "Vector Structure") (Normal :type "Vector Structure") (BoneName :type Name) (PhysMat :type "PhysicalMaterial Object Reference"))
  (bind _bp_player_character (`/Game/Blueprints/Common/MacroLibrary.MGetPlayerCharacter`))
  (`GameplayStatics.ApplyRadialDamage` (`self.DamagePerHit`) Location (`self.DamageRadius`) "/Script/Engine.DamageType" (`|MakeArray` _bp_player_character :!type "Actor Object Reference") null null true))

(fn `OnPhysicsEnd`
  ;[1 1 1] Resets interact symbol offset after physics simulation
  (`SceneComponent.K2_SetWorldLocationAndRotation` :`self` (`self.Billboard`) :`NewLocation` (+ (`SceneComponent.K2_GetComponentLocation` (`self.StaticMesh`)) (`self.InteractOffset`)))
  (set `self.InMotion` false)
  (set `self.CanUse` true)
  (`self.CheckOverlap`))

(fn `SaveState`
  (returns (Data :type "/Game/Blueprints/Common/Structs/SaveableData Structure"))
  (return (make `/Game/Blueprints/Common/Structs/SaveableData` (`KismetStringLibrary.Conv_StringToName` (`KismetSystemLibrary.GetObjectName` self)) (`SceneComponent.K2_GetComponentToWorld` (`self.RootComponent`)))))

(fn `UserConstructionScript`
  (`parent.UserConstructionScript`))