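; BrightnessFade is a Level 3 actor that fades the player's brightness to neutral when play begins.
; On BeginPlay it stores the exposure compensation from the player character's post-process component, reached through the game instance, and waits briefly.
; A timeline then lerps that exposure compensation from the stored value to zero, and the actor destroys itself when it finishes.
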(event `self.ReceiveBeginPlay`
  (bind _bp_game_instance (`/Game/Blueprints/Common/MacroLibrary.MGetGameInstance`))
  (bind _settings (`PostProcessComponent.Settings` (`/Game/Blueprints/Player/BP_PlayerCharacter.PostProcess` (`/Game/Blueprints/Player/BP_GameInstance.PlayerCharacterRef` _bp_game_instance))))
  (bind _output_get (set `self.BeginValue` (`.AutoExposureBias` (break `PostProcessSettings` _settings))))
  (`KismetSystemLibrary.Delay` 2.0)
  (bind (_direction _alpha) (`Timeline|Fade` :!via `PlayFromStart`)
    (:`Update`
      (setmembers `PostProcessSettings` :`StructRef` _settings :`AutoExposureBias` (`KismetMathLibrary.Lerp` _output_get 0.0 _alpha)))
    (:`Finished`
      (`self.K2_DestroyActor`))))

(fn `UserConstructionScript`)