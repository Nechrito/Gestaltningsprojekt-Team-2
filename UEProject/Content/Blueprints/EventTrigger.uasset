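; Overlap trigger actor that fires an event on a linked ITriggerable object when BP_PlayerCharacter enters it.
; Global flags in the game instance gate it, with an optional list that must all be set and an optional flag that blocks it.
; It can also fire only once or require the player to face roughly along its Arrow, using a dot product.
; After calling TriggerEvent on the target, it can set a global flag.
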(event `self.ReceiveBeginPlay`
  (bind _bp_game_instance (`/Game/Blueprints/MacroLibrary.MGetGameInstance`))
  (set `self.GameInstanceRef` _bp_game_instance))

(event `self.ReceiveActorBeginOverlap`
  (params (OtherActor :type "Actor Object Reference"))
  (bind _triggerableobject (`self.TriggerableObject`))
  (if (not (and (`self.TriggerOnlyOnce`) (`self.Triggered`)))
    (bind _continue (`self.CheckFlags`))
    (if _continue
      (if (`self.DoNotTriggerIfGlobalFlagExists`)
        (bind _flagexists (`/Game/Blueprints/Player/BP_GameInstance.CheckGlobalFlag` (`self.GameInstanceRef`) (`self.GlobalFlagToCheck`)))
        (if (not _flagexists)
          (bind _asbp_player_character (cast `/Game/Blueprints/Player/BP_PlayerCharacter` OtherActor :!label _label))
          (if (`self.LimitToDirection`)
            (if (> (`KismetMathLibrary.Dot_VectorVector` (`SceneComponent.GetForwardVector` (`self.Arrow`)) (`self.GetActorForwardVector` _asbp_player_character)) 0.0)
              (set `self.Triggered` true :!label _label_2)
              (`/Engine/EditorBlueprintResources/StandardMacros.IsValid` _triggerableobject
                (:`Is Valid`
                  (bind _asitriggerable (cast `/Game/Blueprints/ITriggerable` _triggerableobject))
                  (`/Game/Blueprints/ITriggerable.TriggerEvent` _asitriggerable self)
                  (if (`self.SetGlobalFlagOnTrigger`)
                    (`/Game/Blueprints/Player/BP_GameInstance.SetGlobalFlag` (`self.GameInstanceRef`) (`self.GlobalFlagToSet`))))))
            (else
              (goto _label_2))))
        (else
          (goto _label))))))

(fn `CheckFlags`
  (returns (Continue :type Boolean))
  (bind _globalflagstocheck (`self.GlobalFlagsToCheck`))
  (if (and (`self.TriggerOnlyIfFlagsExists`) (> (`KismetArrayLibrary.Array_Length` _globalflagstocheck) 0))
    (for _array_element _globalflagstocheck
      (bind _flagexists (`/Game/Blueprints/Player/BP_GameInstance.CheckGlobalFlag` (`self.GameInstanceRef`) _array_element))
      (if (not _flagexists)
        (return false)))
    (return true)
    (else
      (return true))))

(fn `UserConstructionScript`)