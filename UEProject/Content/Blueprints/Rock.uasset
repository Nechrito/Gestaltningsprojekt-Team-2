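; Throwable, saveable rock that the player can grab with the right hand via interaction.
; Throw and Drop flag it as in motion, and Tick waits for near-zero velocities before repositioning the interact billboard, re-enabling use and rechecking overlaps.
; The first hard impact after a throw plays a localized sound and reports an AI noise event, both scaled by impulse.
; Its transform is saved and restored through SaveState and LoadState.
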(event `self.ReceiveBeginPlay`
  (`parent.ReceiveBeginPlay`)
  (`/Game/Blueprints/MacroLibrary.MRegisterSaveable`)
  (bind _bp_game_instance (`/Game/Blueprints/MacroLibrary.MGetGameInstance`))
  (set `self.GameInstanceRef` _bp_game_instance)
  (`KismetSystemLibrary.Delay` 0.2)
  (set `self.InMotion` true))

(event `self.ReceiveTick`
  (params (DeltaSeconds :type "Float (single-precision)"))
  (`parent.ReceiveTick` DeltaSeconds)
  (if (`self.InMotion`)
    (bind _returnvalue (`PrimitiveComponent.GetPhysicsLinearVelocity` (`self.StaticMesh`) "None"))
    (if (and (== _returnvalue (0.0 0.0 0.0) :`ErrorTolerance` 0.01) (== (`PrimitiveComponent.GetPhysicsAngularVelocityInRadians` (`self.StaticMesh`) "None") (0.0 0.0 0.0) :`ErrorTolerance` 0.001))
      (`self.OnPhysicsEnd`))))

(event `/Game/Blueprints/IThrowable.Throw`
  (params (Velocity :type "Vector Structure"))
  (`PrimitiveComponent.SetAllPhysicsLinearVelocity` (`self.StaticMesh`) Velocity true)
  (set `self.InMotion` true)
  (set `self.HasHit` false))

(event `/Game/Blueprints/ISaveable.LoadState`
  (params (Data :type "/Game/Blueprints/SaveableData Structure"))
  (`SceneComponent.K2_SetWorldTransform` (`self.RootComponent`) (`.Transform_17_26866086461CE03CEEE979AE8AEB219A` (break `/Game/Blueprints/SaveableData` Data)) false true))

(event `self.OnInteract`
  (bind _asbp_player_character (cast `/Game/Blueprints/Player/BP_PlayerCharacter` (`GameplayStatics.GetPlayerCharacter` 0)))
  (if (not (`/Game/Blueprints/Player/BP_PlayerCharacter.Grabbing` _asbp_player_character))
    (`/Game/Blueprints/Player/BP_PlayerCharacter.GrabObjectRightHand` :`self` _asbp_player_character :`Location` (`self.K2_GetActorLocation`) :`Object` self)
    (elif (not (`self.CanUse`))
      (set `self.CanUse` true))))

(event `self.StaticMesh.OnComponentHit`
  (params (HitComponent :type "PrimitiveComponent Object Reference") (OtherActor :type "Actor Object Reference") (OtherComp :type "PrimitiveComponent Object Reference") (NormalImpulse :type "Vector Structure") (Hit :type "HitResult Structure (by ref)"))
  (bind _returnvalue (`KismetMathLibrary.VSize` NormalImpulse))
  (bind _returnvalue_2 (`self.K2_GetActorLocation`))
  (bind _returnvalue_3 (`KismetMathLibrary.NormalizeToRange` _returnvalue 0.0 800.0))
  (if (and (> _returnvalue 200.0) (not (`self.HasHit`)))
    (`/Game/Blueprints/Player/BP_GameInstance.PlayLocalizedSound` (`self.GameInstanceRef`) _returnvalue_2 "NewEnumerator0" _returnvalue_3 "NewEnumerator2")
    (set `self.HasHit` true)
    (`AISense_Hearing.ReportNoiseEvent` _returnvalue_2 _returnvalue_3 self 0.0 "Noise")))

(event `/Game/Blueprints/IThrowable.Drop`
  (set `self.InMotion` true)
  (set `self.CanUse` true))

(fn `OnPhysicsEnd`
  ;[1 1 1] Resets interact symbol offset after physics simulation
  (`SceneComponent.K2_SetWorldLocationAndRotation` :`self` (`self.Billboard`) :`NewLocation` (+ (`SceneComponent.K2_GetComponentLocation` (`self.StaticMesh`)) (`self.InteractOffset`)))
  (set `self.InMotion` false)
  (set `self.CanUse` true)
  (`self.CheckOverlap`))

(fn `SaveState`
  (returns (Data :type "/Game/Blueprints/SaveableData Structure"))
  (return (make `/Game/Blueprints/SaveableData` (`KismetStringLibrary.Conv_StringToName` (`KismetSystemLibrary.GetObjectName` self)) (`SceneComponent.K2_GetComponentToWorld` (`self.RootComponent`)))))

(fn `UserConstructionScript`
  (`parent.UserConstructionScript`))