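; AntiWaterBox is a trigger volume that resists the player approaching its center by lowering their MovementModifier, apparently to keep them out of water.
; Overlap events flag the player as inside and cache the current modifier.
; While inside, Tick uses a dot product to scale the modifier by distance over TotalDistance when facing the center, restoring the cached value when facing away.
; An older half-speed implementation remains unconnected.
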(event `self.ReceiveBeginPlay`
  (bind _returnvalue (`GameplayStatics.GetActorOfClass` "/Game/Blueprints/Player/BP_PlayerCharacter.BP_PlayerCharacter_C"))
  (set `self.PlayerRef` _returnvalue))

(event `self.ReceiveTick`
  (params (DeltaSeconds :type "Float (single-precision)"))
  (if (`self.IsInside`)
    (if (>= (`KismetMathLibrary.Dot_VectorVector` (`KismetMathLibrary.Normal` (- (`self.K2_GetActorLocation`) (`self.K2_GetActorLocation` (`self.PlayerRef`)))) (`KismetMathLibrary.Normal` (`self.GetActorForwardVector` (`self.PlayerRef`)))) 0.0)
      (set `/Game/Blueprints/Player/BP_PlayerCharacter.MovementModifier` (`KismetMathLibrary.FClamp` (/ (`KismetMathLibrary.Vector_Distance` (`self.K2_GetActorLocation` self) (`self.K2_GetActorLocation` (`self.PlayerRef`))) (`self.TotalDistance`)) 0.0) (`self.PlayerRef`))
      (else
        (set `/Game/Blueprints/Player/BP_PlayerCharacter.MovementModifier` (`self.CachedSpeed`) (`self.PlayerRef`))))))

(event `self.ReceiveActorBeginOverlap`
  (params (OtherActor :type "Actor Object Reference"))
  (if (== OtherActor (`self.PlayerRef`))
    (set `self.IsInside` true)
    (set `self.CachedSpeed` (`/Game/Blueprints/Player/BP_PlayerCharacter.MovementModifier` (`self.PlayerRef`)))))

(event `self.ReceiveActorEndOverlap`
  (params (OtherActor :type "Actor Object Reference"))
  (if (== OtherActor (`self.PlayerRef`))
    (set `self.IsInside` false)))

(fn `UserConstructionScript`)