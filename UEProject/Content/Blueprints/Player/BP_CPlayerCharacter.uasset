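; Player character Blueprint that handles sprinting, toggled crouching and movement-based camera head bob.
; Sprint input swaps max walk speed while held, with speeds initialised on BeginPlay.
; Crouch input plays or reverses an eased Timeline that lerps capsule half-height between standing and crouched, updating walk speed, rather than calling built-in Crouch.
; Tick plays a sprint, sneak or walk camera shake while the character has velocity and can jump.
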(event `self.ReceiveBeginPlay`
  (set `self.StandingHalfHeight` (`CapsuleComponent.CapsuleHalfHeight` (`self.CapsuleComponent`)))
  (bind _output_get (set `self.WalkSpeed` 200.0)) ; Walk Speed
  (set `CharacterMovementComponent.MaxWalkSpeed` _output_get (`self.CharacterMovement`))
  (set `self.SprintSpeed` 400.0) ; Sprint Speed
  (set `self.CrouchWalkSpeed` 70.0) ; Crouch Walk Speed
)

(event `InputAction|Sprint`
  (params (Key :type "Key Structure"))
  (bind _charactermovement (`self.CharacterMovement`))
  ;[1 1 1] Sprint
  (:`Pressed`
    (set `self.Sprinting` true)
    (set `CharacterMovementComponent.MaxWalkSpeed` (`self.SprintSpeed`) _charactermovement))
  (:`Released`
    (set `self.Sprinting` false)
    (set `CharacterMovementComponent.MaxWalkSpeed` (`self.WalkSpeed`) _charactermovement)))

(event `InputAction|Crouch`
  (params (Key :type "Key Structure"))
  (bind _crouching (`self.Crouching`))
  (bind _charactermovement (`self.CharacterMovement`))
  ;[1 1 1] Crouching
  (:`Pressed`
    (if _crouching
      (set `self.Crouching` false)
      (bind (_direction _easeinout) (`Timeline|CrouchTimeline` :!via `Reverse` :!label _label)
        (:`Update`
          (`CapsuleComponent.SetCapsuleHalfHeight` (`self.CapsuleComponent`) (`KismetMathLibrary.Lerp` (`self.StandingHalfHeight`) (`CharacterMovementComponent.CrouchedHalfHeight` _charactermovement) _easeinout) true)
          (if _crouching
            (set `CharacterMovementComponent.MaxWalkSpeed` (`self.CrouchWalkSpeed`) _charactermovement)
            (else
              (set `CharacterMovementComponent.MaxWalkSpeed` (`self.WalkSpeed`) _charactermovement)))))
      (else
        (set `self.Crouching` true)
        (goto _label)))))

(event `self.ReceiveTick`
  (params (DeltaSeconds :type "Float (single-precision)"))
  (`self.HeadBob`))

(event `HeadBob`
  (bind _returnvalue (`GameplayStatics.GetPlayerController` 0))
  (bind _headbobamount (`self.HeadBobAmount`))
  ;[1 1 1] Headbobbing
  (if (and (> (`KismetMathLibrary.VSizeSquared` (`self.GetVelocity`)) 0.0) (`self.CanJump`))
    (if (`self.Sprinting`)
      (`PlayerController.ClientStartCameraShake` :`self` _returnvalue :`Shake` "/Game/Blueprints/Player/BP_PlayerSprintBob.BP_PlayerSprintBob_C" :`Scale` _headbobamount) ; Sprint
      (elif (`self.Crouching`)
        (`PlayerController.ClientStartCameraShake` :`self` _returnvalue :`Shake` "/Game/Blueprints/Player/BP_PlayerSneakBob.BP_PlayerSneakBob_C" :`Scale` _headbobamount) ; Sneak
        (else
          (`PlayerController.ClientStartCameraShake` :`self` _returnvalue :`Shake` "/Game/Blueprints/Player/BP_PlayerWalkBob.BP_PlayerWalkBob_C" :`Scale` _headbobamount) ; Walk
        )))))

(fn `UserConstructionScript`)