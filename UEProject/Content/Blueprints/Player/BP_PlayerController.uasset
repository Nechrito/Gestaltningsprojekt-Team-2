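; Player controller Blueprint that applies the player's saved look sensitivity and axis inversion settings to camera input.
; On BeginPlay it casts the game instance to BP_GameInstance, caches its save object and calls UpdateControls.
; UpdateControls sets the yaw and pitch input scales from each axis's maximum sensitivity times the saved sensitivity, negated when that axis is inverted.
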(event `self.ReceiveBeginPlay`
  ;[1 1 1] Init
  (bind _asbp_game_instance (cast `/Game/Blueprints/Player/BP_GameInstance` (`GameplayStatics.GetGameInstance`)))
  (set `self.SaveGameInstance` (`/Game/Blueprints/Player/BP_GameInstance.SaveGameInstance` _asbp_game_instance))
  (`self.UpdateControls`))

(event `UpdateControls`
  (bind _savegameinstance (`self.SaveGameInstance`))
  (bind _settingslooksensitivity (`/Game/Blueprints/Player/BP_SaveGame.SettingsLookSensitivity` _savegameinstance))
  (bind _returnvalue (* (`self.MaxSensitivityY`) _settingslooksensitivity))
  (bind _returnvalue_2 (* (`self.MaxSensitivityX`) _settingslooksensitivity))
  ;[1 1 1] Update Controls
  (`|ExecutionSequence`
    (:`then_0`
      (if (`/Game/Blueprints/Player/BP_SaveGame.SettingsInvertXAxis` _savegameinstance)
        (set `self.InputYawScale` (* _returnvalue_2 -1.0))
        (else
          (set `self.InputYawScale` _returnvalue_2))))
    (:`then_1`
      (if (`/Game/Blueprints/Player/BP_SaveGame.SettingsInvertYAxis` _savegameinstance)
        (set `self.InputPitchScale` (* _returnvalue -1.0))
        (else
          (set `self.InputPitchScale` _returnvalue))))))

(fn `UserConstructionScript`)