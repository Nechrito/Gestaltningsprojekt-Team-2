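; Player camera modifier that adjusts the view for zoom and aiming.
; It slides the camera along its forward vector by ZoomModifier and a negative AimAmount offset, and applies a small AimAmount-scaled pitch in view-local space.
; The output FOV is DefaultFOV scaled by FOVModifier, replacing the incoming value.
; An unconnected node that would shift LeftHand by the same zoom and aim offset never runs.
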(fn `BlueprintModifyCamera`
  (params (DeltaTime :type "Float (double-precision)") (ViewLocation :type "Vector Structure") (ViewRotation :type "Rotator Structure") (FOV :type "Float (double-precision)"))
  (returns (NewViewLocation :type "Vector Structure") (NewViewRotation :type "Rotator Structure") (NewFOV :type "Float (double-precision)"))
  (bind _aimamount (`self.AimAmount`))
  (return (+ ViewLocation (* (`KismetMathLibrary.GetForwardVector` ViewRotation) (+ (`self.ZoomModifier`) (* _aimamount -25.0)))) (`KismetMathLibrary.ComposeRotators` (`KismetMathLibrary.RotatorFromAxisAndAngle` (0.0 1.0 0.0) (* _aimamount -2.0)) ViewRotation) (* (`self.DefaultFOV`) (`self.FOVModifier`))))