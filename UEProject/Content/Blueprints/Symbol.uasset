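; Symbol is a saveable, interactable object that the player picks up with the left hand.
; On interaction it passes itself to the player character's left-hand grab through the cached game instance.
; Its trigger event disables further use and sets a global flag on the game instance.
; It registers as saveable on BeginPlay, saving its root transform under its object name and restoring it by teleport on load.
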(event `self.ReceiveBeginPlay`
  (`parent.ReceiveBeginPlay`)
  (`/Game/Blueprints/MacroLibrary.MRegisterSaveable`)
  (bind _bp_game_instance (`/Game/Blueprints/MacroLibrary.MGetGameInstance`))
  (set `self.GameInstanceRef` _bp_game_instance))

(event `self.ReceiveTick`
  (params (DeltaSeconds :type "Float (single-precision)"))
  (`parent.ReceiveTick` DeltaSeconds))

(event `/Game/Blueprints/ISaveable.LoadState`
  (params (Data :type "/Game/Blueprints/SaveableData Structure"))
  (`SceneComponent.K2_SetWorldTransform` (`self.RootComponent`) (`.Transform_17_26866086461CE03CEEE979AE8AEB219A` (break `/Game/Blueprints/SaveableData` Data)) false true))

(event `self.OnInteract`
  (`/Game/Blueprints/Player/BP_PlayerCharacter.GrabObjectLeftHand` (`/Game/Blueprints/Player/BP_GameInstance.PlayerCharacterRef` (`self.GameInstanceRef`)) (`self.K2_GetActorLocation`) self))

(event `/Game/Blueprints/ITriggerable.TriggerEvent`
  (params (TriggerObject :type "/Game/Blueprints/EventTrigger Object Reference"))
  (set `self.CanUse` false)
  (`/Game/Blueprints/Player/BP_GameInstance.SetGlobalFlag` (`self.GameInstanceRef`) (`self.GlobalFlag`)))

(fn `SaveState`
  (returns (Data :type "/Game/Blueprints/SaveableData Structure"))
  (return (make `/Game/Blueprints/SaveableData` (`KismetStringLibrary.Conv_StringToName` (`KismetSystemLibrary.GetObjectName` self)) (`SceneComponent.K2_GetComponentToWorld` (`self.RootComponent`)))))

(fn `UserConstructionScript`
  (`parent.UserConstructionScript`))