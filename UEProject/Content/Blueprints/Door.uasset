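; Interactable door that toggles between closed and open on OnInteract, playing a localized sound through the game instance.
; BeginPlay combines the initial world rotation with the OpenRotation offset and sets both timeline play rates from OpenSpeed.
; The DoorOpenClose timeline plays or reverses to lerp the door's rotation, with collision off until it finishes.
; Opening also runs the HandleTurn timeline to rotate the handle mesh.
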(event `self.ReceiveBeginPlay`
  (bind _openspeed (`self.OpenSpeed`))
  (`parent.ReceiveBeginPlay`)
  (`TimelineComponent.SetPlayRate` (`self.DoorOpenClose`) _openspeed)
  (`TimelineComponent.SetPlayRate` (`self.HandleTurn`) _openspeed)
  (bind _bp_game_instance (`/Game/Blueprints/MacroLibrary.MGetGameInstance`))
  (set `self.GameInstanceRef` _bp_game_instance)
  (bind _output_get (set `self.InitialRotation` (`SceneComponent.K2_GetComponentRotation` (`self.StaticMesh`))))
  (set `self.OpenRotation` (`KismetMathLibrary.ComposeRotators` _output_get (`self.OpenRotation`))))

(event `self.OnInteract`
  (bind _gameinstanceref (`self.GameInstanceRef`))
  (bind _staticmesh (`self.StaticMesh`))
  (`PrimitiveComponent.SetCollisionEnabled` _staticmesh "NoCollision")
  (if (`self.IsOpen`)
    (`/Game/Blueprints/Player/BP_GameInstance.Play Localized Sound` _gameinstanceref (0.0 0.0 0.0) "NewEnumerator1" 1.0 "NewEnumerator2")
    (set `self.IsOpen` false)
    (bind (_direction _float) (`Timeline|DoorOpenClose` :!via `Reverse` :!label _label)
      (:`Update`
        (`SceneComponent.K2_SetWorldRotation` (`self.StaticMesh`) (`KismetMathLibrary.RLerp` (`self.InitialRotation`) (`self.OpenRotation`) _float true) false false))
      (:`Finished`
        (`PrimitiveComponent.SetCollisionEnabled` _staticmesh "QueryAndPhysics")))
    (else
      (`/Game/Blueprints/Player/BP_GameInstance.Play Localized Sound` _gameinstanceref (`self.K2_GetActorLocation` self) "NewEnumerator1" 1.0 "NewEnumerator2")
      (set `self.IsOpen` true)
      (`|ExecutionSequence`
        (:`then_0`
          (bind (_direction_2 _float_2) (`Timeline|HandleTurn` :!via `PlayFromStart`)
            (:`Update`
              (`SceneComponent.K2_SetRelativeRotation` (`self.HandleMesh`) (`KismetMathLibrary.RLerp` (struct :`Roll` 270.0) (struct :`Yaw` 120.0 :`Roll` 180.0) _float_2 true) false false))))
        (:`then_1`
          (goto _label))))))

(fn `UserConstructionScript`
  (`parent.UserConstructionScript`))