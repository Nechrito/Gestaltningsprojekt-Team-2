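; Level 1 loader actor that hands a trigger on to the Tunnel actor and opens up the pool bottom.
; TriggerEvent arms a flag, so Tick polls for a valid Tunnel actor by class until one exists.
; Once found, it fires the Tunnel's TriggerEvent, stops searching, hides PoolBottom and disables its collision, with debug prints marking both stages.
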(event `self.ReceiveTick`
  (params (DeltaSeconds :type "Float (single-precision)"))
  (bind _poolbottom (`self.PoolBottom`))
  (if (`self.LookForTunnel`)
    (bind _returnvalue (`GameplayStatics.GetActorOfClass` "/Game/Blueprints/Level_1/Tunnel.Tunnel_C"))
    (if (`KismetSystemLibrary.IsValid` _returnvalue)
      (`/Game/Blueprints/Level_1/Tunnel.TriggerEvent` _returnvalue null)
      (set `self.LookForTunnel` false)
      (`SceneComponent.SetVisibility` (`Actor.RootComponent` _poolbottom) false false)
      (`PrimitiveComponent.SetCollisionEnabled` (`StaticMeshActor.StaticMeshComponent` _poolbottom) "NoCollision")
      (`KismetSystemLibrary.PrintString` "Found!"))))

(event `/Game/Blueprints/Common/Interfaces/ITriggerable.TriggerEvent`
  (params (TriggerObject :type "/Game/Blueprints/Common/EventTrigger Object Reference"))
  (set `self.LookForTunnel` true)
  (`KismetSystemLibrary.PrintString` "Looking"))

(fn `UserConstructionScript`)