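; ObjectMover is a Level 1 Blueprint that changes the scene in two successive stages as TriggerEvent is called.
; An event counter selects each stage, which updates the WaterController surface, teleports that stage's listed actors to paired locations and unhides its listed objects with their children.
; The counter advances after each stage, and later calls have no matching case.
; BeginPlay caches a game instance reference that the graph never uses.
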(event `self.ReceiveBeginPlay`
  (bind _bp_game_instance (`/Game/Blueprints/Common/MacroLibrary.MGetGameInstance`))
  (set `self.GameInstanceRef` _bp_game_instance))

(event `/Game/Blueprints/Common/Interfaces/ITriggerable.TriggerEvent`
  (params (TriggerObject :type "/Game/Blueprints/Common/EventTrigger Object Reference"))
  (bind _watercontroller (`self.WaterController`))
  (switch `int` (`self.EventCounter`)
    (:`0`
      (`/Game/Blueprints/Common/WaterController.UpdateSurface` _watercontroller)
      (for _array_element (`self.MoveObjects1`)
        (bind (_actor _location) (break `/Game/Blueprints/Common/Structs/ActorLocation` _array_element))
        (`self.K2_SetActorLocation` _actor _location false true))
      (for _array_element_2 (`self.UnhideObjects1`)
        (`SceneComponent.SetVisibility` (`Actor.RootComponent` _array_element_2) true true)))
    (:`1`
      (`/Game/Blueprints/Common/WaterController.UpdateSurface` _watercontroller)
      (for _array_element_3 (`self.MoveObjects2`)
        (bind (_actor_2 _location_2) (break `/Game/Blueprints/Common/Structs/ActorLocation` _array_element_3))
        (`self.K2_SetActorLocation` _actor_2 _location_2 false true))
      (for _array_element_4 (`self.UnhideObjects2`)
        (`SceneComponent.SetVisibility` (`Actor.RootComponent` _array_element_4) true true))))
  (`/Engine/EditorBlueprintResources/StandardMacros.IncrementInt` (`self.EventCounter`)))

(fn `UserConstructionScript`)