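; Interactable wall or surface scribble decal that the player wipes with a held Cloth, enabled when they overlap while holding one.
; Interacting stops player movement and lerps the physics-suspended cloth to the wipe start.
; A second timeline then moves it along WipeNode offsets, driving decal Alpha and CrossFade, before restoring movement and physics.
; BeginPlay shows the wiped state if GlobalFlagName is set, though wiping sets flag "None".
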(event `self.ReceiveBeginPlay`
  (bind _dynamicmaterial (`self.DynamicMaterial`))
  (`parent.ReceiveBeginPlay`)
  (bind _asbp_game_instance (cast `/Game/Blueprints/Player/BP_GameInstance` (`GameplayStatics.GetGameInstance`)))
  (set `self.GameInstanceRef` _asbp_game_instance)
  (set `self.WipeLocation` (`KismetMathLibrary.TransformLocation` (`SceneComponent.K2_GetComponentToWorld` (`self.Scribble`)) (+ (`SceneComponent.RelativeLocation` (`self.WipeNode`)) (`KismetMathLibrary.MakeVector` (* (`self.WipeLength`) 1.0)))))
  (set `self.WipeRotation` (`SceneComponent.K2_GetComponentRotation` (`self.WipeNode`)))
  (bind _returnvalue (`DecalComponent.CreateDynamicMaterialInstance` (`self.ScribbleDecal`)))
  (set `self.DynamicMaterial` _returnvalue)
  (`TimelineComponent.SetPlayRate` (`self.WipeTimeline`) (`self.WipeSpeed`))
  (bind _flagexists (`/Game/Blueprints/Player/BP_GameInstance.CheckGlobalFlag` (`self.GameInstanceRef`) (`self.GlobalFlagName`)))
  (if _flagexists
    (`MaterialInstanceDynamic.SetScalarParameterValue` _dynamicmaterial "CrossFade" 1.0)
    (`MaterialInstanceDynamic.SetScalarParameterValue` _dynamicmaterial "Alpha" 0.4)
    (set `self.CanUse` false)))

(event `self.ReceiveTick`
  (params (DeltaSeconds :type "Float (single-precision)"))
  (`parent.ReceiveTick` DeltaSeconds))

(event `Wipe`
  (bind _dynamicmaterial (`self.DynamicMaterial`))
  (set `/Game/Blueprints/Level_1/ClothAnim.IsWiping` true (`/Game/Blueprints/Level_1/Cloth.ClothAnim` (`self.Cloth`)))
  (`/Game/Blueprints/Player/BP_GameInstance.PlayCharacterSound` (`self.GameInstanceRef`) (`self.WipeNode`) "NewEnumerator26" 1.0 "NewEnumerator8")
  (bind (_direction _alpha _crossfade _wipe) (`Timeline|WipeTimeline` :!via `PlayFromStart`)
    (:`Update`
      (`MaterialInstanceDynamic.SetScalarParameterValue` _dynamicmaterial "Alpha" _alpha)
      (`MaterialInstanceDynamic.SetScalarParameterValue` _dynamicmaterial "CrossFade" _crossfade)
      (`self.K2_SetActorLocation` (`self.Cloth`) (`KismetMathLibrary.TransformLocation` (`SceneComponent.K2_GetComponentToWorld` (`self.Scribble`)) (+ (`SceneComponent.RelativeLocation` (`self.WipeNode`)) (* _wipe (`self.WipeLength`)))) false false))
    (:`Finished`
      (`/Game/Blueprints/Player/BP_GameInstance.SetGlobalFlag` (`self.GameInstanceRef`) "None")
      (`self.EndWipe`))))

(event `self.OnInteract`
  (bind _staticmesh (`/Game/Blueprints/Common/InteractableBase.StaticMesh` (`self.Cloth`)))
  (bind _ascloth (cast `/Game/Blueprints/Level_1/Cloth` (`/Game/Blueprints/Player/BP_PlayerCharacter.HoldableObject` (`/Game/Blueprints/Player/BP_GameInstance.PlayerCharacterRef` (`self.GameInstanceRef`)))))
  (set `self.Cloth` _ascloth)
  (bind _staticmesh_2 (`/Game/Blueprints/Common/InteractableBase.StaticMesh` _ascloth))
  (`PrimitiveComponent.SetEnableGravity` _staticmesh_2 false)
  (`PrimitiveComponent.PutRigidBodyToSleep` _staticmesh_2 "None")
  (set `self.ClothLocation` (`self.K2_GetActorLocation` _ascloth))
  (set `self.ClothRotation` (`self.K2_GetActorRotation` _ascloth))
  (`/Game/Blueprints/Player/BP_PlayerCharacter.SetMovementModifier` (`/Game/Blueprints/Player/BP_GameInstance.PlayerCharacterRef` (`self.GameInstanceRef`)) 0.0)
  (bind (_direction _alpha) (`Timeline|Timeline_0` :!via `PlayFromStart`)
    (:`Update`
      (`self.K2_SetActorLocationAndRotation` (`self.Cloth`) (`KismetMathLibrary.VLerp` (`self.ClothLocation`) (`self.WipeLocation`) _alpha) (`KismetMathLibrary.RLerp` (`self.ClothRotation`) (`self.WipeRotation`) _alpha true) false false))
    (:`Finished`
      (if (`|EnumEquality` _direction "Forward")
        (`self.Wipe`)
        (else
          (`/Game/Blueprints/Player/BP_PlayerCharacter.SetMovementModifier` (`/Game/Blueprints/Player/BP_GameInstance.PlayerCharacterRef` (`self.GameInstanceRef`)) 1.0 :!label _label)
          (`PrimitiveComponent.SetEnableGravity` _staticmesh true)
          (`PrimitiveComponent.WakeRigidBody` _staticmesh "None"))))))

(event `EndWipe`
  (bind _cloth (`self.Cloth`))
  (set `self.ClothLocation` (`self.K2_GetActorLocation` _cloth))
  (set `self.ClothRotation` (`self.K2_GetActorRotation` _cloth))
  (set `/Game/Blueprints/Level_1/ClothAnim.IsWiping` false (`/Game/Blueprints/Level_1/Cloth.ClothAnim` _cloth))
  (goto _label))

(event `self.ReceiveActorBeginOverlap`
  (params (OtherActor :type "Actor Object Reference"))
  (bind _asbp_player_character (cast `/Game/Blueprints/Player/BP_PlayerCharacter` OtherActor)
    (:`then`
      (if (`/Game/Blueprints/Player/BP_PlayerCharacter.HoldingObject` _asbp_player_character)
        (cast `/Game/Blueprints/Level_1/Cloth` (`/Game/Blueprints/Player/BP_PlayerCharacter.HoldableObject` _asbp_player_character)
          (:`then`
            (set `self.Disabled` false))
          (:`CastFailed`
            _))))
    (:`CastFailed`
      _))
  (`parent.ReceiveActorBeginOverlap` OtherActor))

(event `self.ReceiveActorEndOverlap`
  (params (OtherActor :type "Actor Object Reference"))
  (`parent.ReceiveActorEndOverlap` OtherActor))

(fn `UserConstructionScript`)