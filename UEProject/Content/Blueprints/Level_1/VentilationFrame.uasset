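; VentilationFrame is a level actor that moves the player up into a ventilation opening along a spline, once, when they enter its trigger while the Hatch is open.
; The overlap stops player movement and gravity, enables crawling mode and lowers eye height.
; A timeline then teleports the character each update, blending from the entry position onto the spline path and driving gravity scale.
; On finish, movement resumes at a reduced modifier.
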(event `self.ClimbTrigger.OnComponentBeginOverlap`
  (params (OverlappedComponent :type "PrimitiveComponent Object Reference") (OtherActor :type "Actor Object Reference") (OtherComp :type "PrimitiveComponent Object Reference") (OtherBodyIndex :type Integer) (bFromSweep :type Boolean) (SweepResult :type "HitResult Structure (by ref)"))
  (bind _playercharacterref (`self.PlayerCharacterRef`))
  (bind _playercharacterref_2 (`self.PlayerCharacterRef`))
  (bind _charactermovement (`Character.CharacterMovement` (`self.PlayerCharacterRef`)))
  (bind _asbp_player_character (cast `/Game/Blueprints/Player/BP_PlayerCharacter` OtherActor))
  (if (and (`/Game/Blueprints/Common/DoorBase.IsOpen` (`self.Hatch`)) (not (`self.Climbed`)))
    (set `self.Climbed` true)
    (set `self.PlayerCharacterRef` _asbp_player_character)
    (`/Game/Blueprints/Player/BP_PlayerCharacter.SetMovementModifier` _playercharacterref 0.0)
    (set `CharacterMovementComponent.GravityScale` 0.0 _charactermovement)
    (`/Game/Blueprints/Player/BP_PlayerCharacter.SetCrawlingMode` _playercharacterref true)
    (`/Game/Blueprints/Player/BP_PlayerCharacter.SetEyeHeight` _playercharacterref 15.0)
    (set `self.StartLocation` (`self.K2_GetActorLocation` _playercharacterref))
    (bind (_direction _alpha _splinefollow _gravityscale) (`Timeline|ClimbTimeline` :!via `PlayFromStart`)
      (:`Update`
        (set `CharacterMovementComponent.GravityScale` _gravityscale _charactermovement)
        (`self.K2_SetActorLocation` _playercharacterref_2 (`KismetMathLibrary.VLerp` (`self.StartLocation`) (`SplineComponent.GetLocationAtTime` (`self.Spline`) _alpha "World" false) _splinefollow) false true))
      (:`Finished`
        (`/Game/Blueprints/Player/BP_PlayerCharacter.SetMovementModifier` _playercharacterref_2 0.5)))))

(fn `UserConstructionScript`
  (`parent.UserConstructionScript`))