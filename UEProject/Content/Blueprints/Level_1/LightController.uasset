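; Level 1 light controller that runs a scripted lighting sequence with Perlin-noise flicker across roof and pool lights.
; BeginPlay assigns dynamic emissive materials to five mesh groups.
; TriggerEvent runs a player-speed timeline, then a light timeline driving each group's intensity and emissive strength.
; A counter-based Events switch, fired between timelines and by timeline events, selects localized sounds, ObjectMover triggers or a movement-speed reset.
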(event `self.ReceiveBeginPlay`
  (bind _bp_game_instance (`/Game/Blueprints/Common/MacroLibrary.MGetGameInstance`))
  (set `self.GameInstanceRef` _bp_game_instance)
  (bind _returnvalue (`KismetMaterialLibrary.CreateDynamicMaterialInstance` "/Game/Assets/Materials/Level_2/Emisiv_pool_windo_light_Inst.Emisiv_pool_windo_light_Inst"))
  (set `self.Material5` _returnvalue)
  (bind _returnvalue_2 (`KismetMaterialLibrary.CreateDynamicMaterialInstance` "/Game/Assets/Materials/Level_1/Ebmisiv_laps_Lv1_isnt.Ebmisiv_laps_Lv1_isnt"))
  (set `self.Material1` _returnvalue_2)
  (bind _returnvalue_3 (`KismetMaterialLibrary.CreateDynamicMaterialInstance` "/Game/Assets/Materials/Level_1/Ebmisiv_laps_Lv1_isnt.Ebmisiv_laps_Lv1_isnt"))
  (set `self.Material2` _returnvalue_3)
  (bind _returnvalue_4 (`KismetMaterialLibrary.CreateDynamicMaterialInstance` "/Game/Assets/Materials/Level_1/Ebmisiv_laps_Lv1_isnt.Ebmisiv_laps_Lv1_isnt"))
  (set `self.Material3` _returnvalue_4)
  (bind _returnvalue_5 (`KismetMaterialLibrary.CreateDynamicMaterialInstance` "/Game/Assets/Materials/Level_1/Ebmisiv_laps_Lv1_isnt.Ebmisiv_laps_Lv1_isnt"))
  (set `self.Material4` _returnvalue_5)
  (`self.SetMaterialInstances` (`self.MeshGroup1`) (`self.Material1`) 1)
  (`self.SetMaterialInstances` (`self.MeshGroup2`) (`self.Material2`) 1)
  (`self.SetMaterialInstances` (`self.MeshGroup3`) (`self.Material3`) 1)
  (`self.SetMaterialInstances` (`self.MeshGroup4`) (`self.Material4`) 1)
  (`self.SetMaterialInstances` (`self.MeshGroup5`) (`self.Material5`) 1)
  (bind _returnvalue_6 (`MaterialInstanceDynamic.K2_GetScalarParameterValue` (`self.Material1`) "Emissive Strength"))
  (set `self.RoofEmissiveStrength` _returnvalue_6)
  (bind _returnvalue_7 (`MaterialInstanceDynamic.K2_GetScalarParameterValue` (`self.Material5`) "Emissive Strength"))
  (set `self.PoolEmissiveStrength` _returnvalue_7))

(event `/Game/Blueprints/Common/Interfaces/ITriggerable.TriggerEvent`
  (params (TriggerObject :type "/Game/Blueprints/Common/EventTrigger Object Reference"))
  (bind _roofemissivestrength (`self.RoofEmissiveStrength`))
  (bind _returnvalue (`GameplayStatics.GetActorOfClass` "/Game/Blueprints/Level_1/ObjectMover.ObjectMover_C"))
  (set `self.ObjectMoverRef` _returnvalue)
  (bind (_direction _playerspeed) (`Timeline|Timeline_0` :!via `PlayFromStart`)
    (:`Update`
      (`/Game/Blueprints/Player/BP_PlayerCharacter.SetMovementModifier` (`/Game/Blueprints/Player/BP_GameInstance.PlayerCharacterRef` (`self.GameInstanceRef`)) _playerspeed))
    (:`Finished`
      (`self.Events`)
      (bind (_direction_2 _track1 _track2 _track3 _track4 _flicker _time) (`Timeline|LightTimeline` :!via `PlayFromStart`)
        (:`Update`
          (bind _returnvalue_2 (- 1.0 (* (`KismetMathLibrary.PerlinNoise1D` _time) _flicker (`self.FlickerIntensity`))))
          (bind _returnvalue_3 (* _returnvalue_2 (`self.RoofLightIntensity`)))
          (`self.SetLightIntensity` (`self.LightGroup1`) (* _returnvalue_3 _track1))
          (`MaterialInstanceDynamic.SetScalarParameterValue` (`self.Material1`) "Emissive Strength" (* _roofemissivestrength _track1))
          (`self.SetLightIntensity` (`self.LightGroup2`) (* _returnvalue_3 _track2))
          (`MaterialInstanceDynamic.SetScalarParameterValue` (`self.Material2`) "Emissive Strength" (* _roofemissivestrength _track2))
          (`self.SetLightIntensity` (`self.LightGroup3`) (* _returnvalue_3 _track3))
          (`MaterialInstanceDynamic.SetScalarParameterValue` (`self.Material3`) "Emissive Strength" (* _roofemissivestrength _track3))
          (`self.SetLightIntensity` (`self.LightGroup4`) (* _returnvalue_3 _track4))
          (`MaterialInstanceDynamic.SetScalarParameterValue` (`self.Material4`) "Emissive Strength" (* _roofemissivestrength _track4))
          (`self.SetLightIntensity` (`self.LightGroup5`) (* (* _returnvalue_2 (`self.PoolLightIntensity`)) _track4))
          (`MaterialInstanceDynamic.SetScalarParameterValue` (`self.Material5`) "Emissive Strength" (* (`self.PoolEmissiveStrength`) _track4)))
        (:`Events`
          (`self.Events`))))))

(event `Events`
  (switch `int` (`self.EventCounter`)
    (:`0`
      (`/Game/Blueprints/Player/BP_GameInstance.PlayLocalizedSound` (`self.GameInstanceRef`) (0.0 0.0 0.0) "NewEnumerator15" 1.0 "NewEnumerator8" :!label _label)
      (`/Engine/EditorBlueprintResources/StandardMacros.IncrementInt` (`self.EventCounter`)))
    (:`1`
      (goto _label))
    (:`2`
      (`/Game/Blueprints/Common/Interfaces/ITriggerable.TriggerEvent` (`self.ObjectMoverRef`) null :!label _label_2))
    (:`3`
      (goto _label))
    (:`4`
      (goto _label))
    (:`5`
      (`/Game/Blueprints/Player/BP_PlayerCharacter.SetMovementModifier` (`/Game/Blueprints/Player/BP_GameInstance.PlayerCharacterRef` (`self.GameInstanceRef`)) 1.0)
      (goto _label_2))))

(fn `SetLightIntensity`
  (params (Lights :type "Array of Light Object Reference (by ref)") (Intensity :type "Float (double-precision) (by ref)"))
  (for _array_element Lights
    (`LightComponent.SetIntensity` (`Light.LightComponent` _array_element) Intensity)))

(fn `SetMaterialInstances`
  (params (Actors :type "Array of StaticMeshActor Object Reference (by ref)") (Material :type "MaterialInstanceDynamic Object Reference") (Index :type Integer))
  (for _array_element Actors
    (`PrimitiveComponent.SetMaterial` (`StaticMeshActor.StaticMeshComponent` _array_element) Index Material)))

(fn `UserConstructionScript`)