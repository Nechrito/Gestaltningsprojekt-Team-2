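; Central sound dispatcher that plays FMOD events for gameplay, creature and UI sounds.
; On BeginPlay it binds to the game instance's localized-sound and attach-source events, then switches on sound type.
; Localized sounds play at a location or in 2D for UI, while attached sources cover critters, monster and portal pieces.
; Footsteps set a Material parameter, but the surface-to-material switch is unwired, and Intensity is unused.
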(event `self.ReceiveBeginPlay`
  (bind _bp_game_instance (`/Game/Blueprints/Common/MacroLibrary.MGetGameInstance`))
  (bind _output_get (set `self.GameInstanceRef` _bp_game_instance))
  (add `/Game/Blueprints/Player/BP_GameInstance.LocalizedSoundEvent` _output_get (delegate `OnLocalizedSound`))
  (add `/Game/Blueprints/Player/BP_GameInstance.AttachSoundSourceEvent` _output_get (delegate `OnAttachedSoundSource`)))

(event `OnAttachedSoundSource`
  (params (SceneComponent :type "SceneComponent Object Reference") (SoundType :type "/Game/Blueprints/Common/Enum/LocalizedSoundType Enum" :default "NewEnumerator31") (Intensity :type "Float (double-precision)"))
  (switch `/Game/Blueprints/Common/Enum/LocalizedSoundType` SoundType
    (:`NewEnumerator5`
      (`FMODBlueprintStatics.PlayEventAttached` "/Game/FMOD/Events/Critters/Critters_sound.Critters_sound" SceneComponent "None" (0.0 0.0 0.0) "KeepRelativeOffset"))
    (:`NewEnumerator0`
      (`FMODBlueprintStatics.PlayEventAttached` "/Game/FMOD/Events/Monster/Monstersound.Monstersound" SceneComponent "None" (0.0 0.0 0.0) "KeepRelativeOffset"))
    (:`NewEnumerator4`
      (bind _returnvalue (`FMODBlueprintStatics.PlayEventAttached` "/Game/FMOD/Events/Monster/Footsteps.Footsteps" SceneComponent "None" (0.0 0.0 0.0) "KeepRelativeOffset"))
      (`FMODAudioComponent.SetParameter` _returnvalue "Material" (`self.Material`)))
    (:`NewEnumerator1`
      (`FMODBlueprintStatics.PlayEventAttached` "/Game/FMOD/Events/Monster/Shooting_smoke.Shooting_smoke" SceneComponent "None" (0.0 0.0 0.0) "KeepRelativeOffset"))
    (:`NewEnumerator33`
      (`FMODBlueprintStatics.PlayEventAttached` "/Game/FMOD/Events/Object_interactions/Portal_pieces.Portal_pieces" null "None" (0.0 0.0 0.0) "KeepRelativeOffset"))))

(event `OnLocalizedSound`
  (params (Location :type "Vector Structure") (SoundType :type "/Game/Blueprints/Common/Enum/LocalizedSoundType Enum" :default "NewEnumerator31") (Intensity :type "Float (double-precision)") (SurfaceType :type "/Game/Blueprints/Common/Enum/SoundSurfaceType Enum" :default "NewEnumerator8"))
  (bind _returnvalue (`KismetMathLibrary.Conv_VectorToTransform` Location))
  (bind _returnvalue_2 (`KismetMathLibrary.Conv_VectorToTransform` Location))
  (switch `/Game/Blueprints/Common/Enum/LocalizedSoundType` SoundType
    (:`NewEnumerator6`
      (`FMODBlueprintStatics.PlayEventAtLocation` "/Game/FMOD/Events/Object_interactions/Dörrar/Open_locker_room_doors.Open_locker_room_doors" (`KismetMathLibrary.Conv_VectorToTransform` Location)))
    (:`NewEnumerator7`
      (`FMODBlueprintStatics.PlayEventAtLocation` "/Game/FMOD/Events/Object_interactions/Dörrar/Close_Locker_room_doors.Close_Locker_room_doors" (`KismetMathLibrary.Conv_VectorToTransform` Location)))
    (:`NewEnumerator8`
      (`FMODBlueprintStatics.PlayEventAtLocation` "/Game/FMOD/Events/Object_interactions/Dörrar/Going_though_portal.Going_though_portal" (`KismetMathLibrary.Conv_VectorToTransform` Location)))
    (:`NewEnumerator9`
      (`FMODBlueprintStatics.PlayEventAtLocation` "/Game/FMOD/Events/Object_interactions/Dörrar/Gate_till_hopptorn.Gate_till_hopptorn" (`KismetMathLibrary.Conv_VectorToTransform` Location)))
    (:`NewEnumerator10`
      (`FMODBlueprintStatics.PlayEventAtLocation` "/Game/FMOD/Events/Object_interactions/Throwing/Rock_Land_in_water.Rock_Land_in_water" (`KismetMathLibrary.Conv_VectorToTransform` Location)))
    (:`NewEnumerator11`
      (`FMODBlueprintStatics.PlayEventAtLocation` "/Game/FMOD/Events/Object_interactions/Throwing/Rock_Land_on_ground.Rock_Land_on_ground" (`KismetMathLibrary.Conv_VectorToTransform` Location)))
    (:`NewEnumerator12`
      (`FMODBlueprintStatics.PlayEventAtLocation` "/Game/FMOD/Events/Object_interactions/Throwing/Waterballoon_land.Waterballoon_land" _returnvalue))
    (:`NewEnumerator13`
      (`FMODBlueprintStatics.PlayEventAtLocation` "/Game/FMOD/Events/Object_interactions/Dragging_Bench.Dragging_Bench" _returnvalue))
    (:`NewEnumerator14`
      (`FMODBlueprintStatics.PlayEventAtLocation` "/Game/FMOD/Events/Object_interactions/Fail_to_open_locker.Fail_to_open_locker" _returnvalue))
    (:`NewEnumerator18`
      (`FMODBlueprintStatics.PlayEventAtLocation` "/Game/FMOD/Events/Object_interactions/Grab_portal_piece.Grab_portal_piece" (`KismetMathLibrary.Conv_VectorToTransform` Location)))
    (:`NewEnumerator19`
      (`FMODBlueprintStatics.PlayEventAtLocation` "/Game/FMOD/Events/Object_interactions/Place_portal_piece_in_portal.Place_portal_piece_in_portal" (`KismetMathLibrary.Conv_VectorToTransform` Location)))
    (:`NewEnumerator20`
      (`FMODBlueprintStatics.PlayEventAtLocation` "/Game/FMOD/Events/Object_interactions/Plastic_chair_dragging.Plastic_chair_dragging" _returnvalue))
    (:`NewEnumerator21`
      (`FMODBlueprintStatics.PlayEventAtLocation` "/Game/FMOD/Events/Object_interactions/Plastic_chair_release.Plastic_chair_release" _returnvalue))
    (:`NewEnumerator22`
      (`FMODBlueprintStatics.PlayEventAtLocation` "/Game/FMOD/Events/Object_interactions/Water_gun_pick_up.Water_gun_pick_up" _returnvalue))
    (:`NewEnumerator23`
      (`FMODBlueprintStatics.PlayEventAtLocation` "/Game/FMOD/Events/Object_interactions/Water_gun_recharge.Water_gun_recharge" _returnvalue))
    (:`NewEnumerator24`
      (`FMODBlueprintStatics.PlayEventAtLocation` "/Game/FMOD/Events/Object_interactions/Water_gun_squirt.Water_gun_squirt" _returnvalue))
    (:`NewEnumerator32`
      (`FMODBlueprintStatics.PlayEventAtLocation` "/Game/FMOD/Events/Object_interactions/Pick_up_Cloth.Pick_up_Cloth" _returnvalue_2))
    (:`NewEnumerator27`
      (`FMODBlueprintStatics.PlayEvent2D` "/Game/FMOD/Events/UI/Back.Back"))
    (:`NewEnumerator29`
      (`FMODBlueprintStatics.PlayEvent2D` "/Game/FMOD/Events/UI/Enter.Enter"))
    (:`NewEnumerator28`
      (`FMODBlueprintStatics.PlayEvent2D` "/Game/FMOD/Events/UI/Paus_menu.Paus_menu"))
    (:`NewEnumerator30`
      (`FMODBlueprintStatics.PlayEvent2D` "/Game/FMOD/Events/UI/Scrole.Scrole"))
    (:`NewEnumerator34`
      (`FMODBlueprintStatics.PlayEventAtLocation` "/Game/FMOD/Events/Ambience/Spot_Ambience/Shower.Shower" _returnvalue_2))
    (:`NewEnumerator35`
      (`FMODBlueprintStatics.PlayEventAtLocation` "/Game/FMOD/Events/Ambience/Spot_Ambience/Flickering_lights.Flickering_lights" _returnvalue_2))
    (:`NewEnumerator36`
      (`FMODBlueprintStatics.PlayEventAtLocation` "/Game/FMOD/Events/Ambience/Spot_Ambience/Flourescent_light_buzz.Flourescent_light_buzz" _returnvalue_2))
    (:`NewEnumerator37`
      (`FMODBlueprintStatics.PlayEventAtLocation` "/Game/FMOD/Events/Object_interactions/Dörrar/Gate_till_hopptorn_close.Gate_till_hopptorn_close" _returnvalue_2))))

(fn `UserConstructionScript`
  (`parent.UserConstructionScript`))