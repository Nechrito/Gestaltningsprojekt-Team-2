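; Character audio Blueprint that plays sound events, apparently FMOD, in response to character sound broadcasts from the game instance.
; On BeginPlay it binds to the character sound and heartbeat begin/end events.
; Only footsteps are live, played as a plain 2D event; both heartbeat handlers are empty.
; Disconnected logic holds attached heartbeat, run, cough and swimming sounds, plus surface-to-Material parameter mapping for footsteps and running.
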(event `self.ReceiveBeginPlay`
  (bind _bp_game_instance (`/Game/Blueprints/Common/MacroLibrary.MGetGameInstance`))
  (bind _output_get (set `self.GameInstanceRef` _bp_game_instance))
  (add `/Game/Blueprints/Player/BP_GameInstance.CharacterSoundEvent` _output_get (delegate `OnCharacterSound`))
  (add `/Game/Blueprints/Player/BP_GameInstance.BeginHeartbeatSoundEvent` _output_get (delegate `OnHeartbeatBegin`))
  (add `/Game/Blueprints/Player/BP_GameInstance.EndHeartbeatSoundEvent` _output_get (delegate `OnHeartbeatEnd`)))

(event `OnCharacterSound`
  (params (SceneComponent :type "SceneComponent Object Reference") (SoundType :type "/Game/Blueprints/Common/Enum/CharacterSoundType Enum" :default "NewEnumerator0") (Intensity :type "Float (double-precision)") (SurfaceType :type "/Game/Blueprints/Common/Enum/SoundSurfaceType Enum" :default "NewEnumerator8"))
  (set `self.Location` (`SceneComponent.K2_GetComponentLocation` SceneComponent))
  (switch `/Game/Blueprints/Common/Enum/CharacterSoundType` SoundType
    (:`NewEnumerator0`
      (`FMODBlueprintStatics.PlayEvent2D` "/Game/FMOD/Events/Character/Footsteps/Footsteps.Footsteps"))))

(event `OnHeartbeatBegin`)

(event `OnHeartbeatEnd`)

(event `self.ReceiveTick`
  (params (DeltaSeconds :type "Float (single-precision)")))

(fn `UserConstructionScript`
  (`parent.UserConstructionScript`))