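; Sound manager that plays music for the menu, Level 1 and Level 3 on request from the game instance.
; On BeginPlay it binds to the game instance's music, sound level and level restart events; the latter two handlers are empty.
; A new music type starts a 2D FMOD event, or stops the current one if unmapped.
; Intensity is passed as an event parameter, with inconsistent parameter names across branches.
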(event `self.ReceiveBeginPlay`
  (bind _bp_game_instance (`/Game/Blueprints/Common/MacroLibrary.MGetGameInstance`))
  (bind _output_get (set `self.GameInstanceRef` _bp_game_instance))
  (add `/Game/Blueprints/Player/BP_GameInstance.PlayMusicEvent` _output_get (delegate `OnPlayMusic`))
  (add `/Game/Blueprints/Player/BP_GameInstance.SetSoundLevelsEvent` _output_get (delegate `OnSetSoundLevels`))
  (add `/Game/Blueprints/Player/BP_GameInstance.LevelRestartEvent` _output_get (delegate `OnLevelRestart`)))

(event `OnPlayMusic`
  (params (MusicType :type "/Game/Blueprints/Common/Enum/MusicType Enum" :default "NewEnumerator0") (Intensity :type "Float (double-precision)"))
  (bind _currentevent (`self.CurrentEvent`))
  (if (`|EnumInequality` (`self.MusicCurrentlyPlaying`) MusicType)
    (bind _output_get (set `self.MusicCurrentlyPlaying` MusicType))
    (switch `/Game/Blueprints/Common/Enum/MusicType` _output_get
      (:`NewEnumerator0`
        (`FMODBlueprintStatics.EventInstanceStop` (`self.CurrentEvent`)))
      (:`NewEnumerator1`
        (bind _returnvalue (`FMODBlueprintStatics.PlayEvent2D` "/Game/FMOD/Events/UI/meny.meny"))
        (bind _output_get_2 (set `self.CurrentEvent` _returnvalue))
        (`FMODBlueprintStatics.EventInstanceSetParameter` _output_get_2 "Intensity" Intensity))
      (:`NewEnumerator2`
        (bind _returnvalue_2 (`FMODBlueprintStatics.PlayEvent2D` "/Game/FMOD/Events/Musik/lvl_3_(Badhuset_fight).lvl_3_(Badhuset_fight)"))
        (bind _output_get_3 (set `self.CurrentEvent` _returnvalue_2))
        (`FMODBlueprintStatics.EventInstanceSetParameter` _output_get_3 "Intensity" Intensity))
      (:`NewEnumerator3`
        (bind _returnvalue_3 (`FMODBlueprintStatics.PlayEvent2D` "/Game/FMOD/Events/Musik/lvl_1_(Badhuset).lvl_1_(Badhuset)"))
        (bind _output_get_4 (set `self.CurrentEvent` _returnvalue_3))
        (`FMODBlueprintStatics.EventInstanceSetParameter` _output_get_4 "Parameter 1" Intensity)))
    (else
      (switch `/Game/Blueprints/Common/Enum/MusicType` MusicType
        (:`NewEnumerator1`
          (`FMODBlueprintStatics.EventInstanceSetParameter` _currentevent "Parameter 1" Intensity))
        (:`NewEnumerator2`
          (`FMODBlueprintStatics.EventInstanceSetParameter` _currentevent "Parameter 1" Intensity))
        (:`NewEnumerator3`
          (`FMODBlueprintStatics.EventInstanceSetParameter` _currentevent "Parameter 1" Intensity))))))

(event `OnSetSoundLevels`
  (params (MasterVolume :type "Float (double-precision)") (SoundEffectVolume :type "Float (double-precision)") (MusicVolume :type "Float (double-precision)")))

(event `OnLevelRestart`)

(fn `UserConstructionScript`
  (`parent.UserConstructionScript`))